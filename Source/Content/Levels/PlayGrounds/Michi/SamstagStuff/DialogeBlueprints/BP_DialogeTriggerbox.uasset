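; Dialogue trigger box that plays a one-time 2D voice or sound cue with a dialogue widget when BP_Player overlaps it.
; An optional collectables collection gates it: CanPlay is set through its all-collected event binding, while an unassigned collection lets it play immediately.
; On firing, it removes the box, shows WBP_Dialoge for the cue's duration, then removes the widget and destroys itself.
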(event OnComponentBeginOverlap(Box)
  (params (OverlappedComponent :type Primitive%20Component%20Object%20Reference) (OtherActor :type Actor%20Object%20Reference) (OtherComp :type Primitive%20Component%20Object%20Reference) (OtherBodyIndex :type Integer) (bFromSweep :type Boolean) (SweepResult :type Hit%20Result%20Structure%20%28by%20ref%29))
  (bind _soundcue (Variables|Default|GetSoundcue))
  (bind _asbp_player (Utilities|Casting|CastToBP_Player OtherActor))
  (Utilities|IsValid _asbp_player
    (:Is%20Valid
      (Utilities|IsValid (Variables|Default|GetCollectionOfColletabels)
        (:Is%20Valid
          (if (Variables|Default|GetcanPlay)
            (Components|DestroyComponent (Variables|Default|GetBox) :!label _label)
            (bind _returnvalue (UserInterface|CreateWidget "/Game/Levels/PlayGrounds/Michi/SamstagStuff/Widget/WBP_Dialoge.WBP_Dialoge_C"))
            (UserInterface|Viewport|AddtoViewport _returnvalue 0)
            (Audio|PlaySound2D _soundcue 1.0 1.0 0.0 0 0)
            (Utilities|FlowControl|Delay (Variables|/Script/Engine.SoundBase|GetDuration _soundcue))
            (Widget|RemovefromParent _returnvalue)
            (Actor|DestroyActor)))
        (:Is%20Not%20Valid
          (goto _label))))))

(event Custom|OnAllCollectable
  (Variables|Default|SetcanPlay true))

(event EventBeginPlay
  (bind _collectionofcolletabels (Variables|Default|GetCollectionOfColletabels))
  (Utilities|IsValid _collectionofcolletabels
    (:Is%20Valid
      (EventDispatchers|BindEventtoOnAllCollected _collectionofcolletabels (EventDispatchers|CreateEvent :!event Custom|OnAllCollectable)))))

(fn ConstructionScript)