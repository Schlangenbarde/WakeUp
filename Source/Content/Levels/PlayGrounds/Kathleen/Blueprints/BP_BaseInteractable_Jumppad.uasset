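; Heat-reactive jump pad interactable that launches BP_Player into a high jump while in one specific heat state.
; Switching to hot makes the cube block pawns, while cold makes it overlap them, each swapping material and optionally playing a sound.
; Overlapping triggers the player's frozen-ground behavior, and leaving clears it.
; Both hits and overlap exits attempt the state-gated jump.
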(event OnComponentEndOverlap(Cube)
  (params (OverlappedComponent :type Primitive%20Component%20Object%20Reference) (OtherActor :type Actor%20Object%20Reference) (OtherComp :type Primitive%20Component%20Object%20Reference) (OtherBodyIndex :type Integer))
  (bind _asbp_player (Utilities|Casting|CastToBP_Player OtherActor))
  (Default|PerformUnfrozen _asbp_player)
  (CallFunction|MakePlayerPerformHighJump _asbp_player))

(event OnComponentBeginOverlap(Cube)
  (params (OverlappedComponent :type Primitive%20Component%20Object%20Reference) (OtherActor :type Actor%20Object%20Reference) (OtherComp :type Primitive%20Component%20Object%20Reference) (OtherBodyIndex :type Integer) (bFromSweep :type Boolean) (SweepResult :type Hit%20Result%20Structure%20%28by%20ref%29))
  (bind _asbp_player (Utilities|Casting|CastToBP_Player OtherActor))
  (Default|PerformFrozenGround _asbp_player))

(event OnComponentHit(Cube)
  (params (HitComponent :type Primitive%20Component%20Object%20Reference) (OtherActor :type Actor%20Object%20Reference) (OtherComp :type Primitive%20Component%20Object%20Reference) (NormalImpulse :type Vector :default "0, 0, 0") (Hit :type Hit%20Result%20Structure%20%28by%20ref%29))
  (bind _asbp_player (Utilities|Casting|CastToBP_Player OtherActor))
  (CallFunction|MakePlayerPerformHighJump _asbp_player))

(fn ConstructionScript
  (|CallParentFunction))

(fn Interact
  (params (incomingHeat :type ENUM_HeatState%20Enum :default "NewEnumerator13"))
  (|CallParentFunction incomingHeat))

(fn SwitchtoColdState
  (params (shouldplaySound :type Boolean))
  (bind _cube (Variables|Default|GetCube))
  (if shouldplaySound
    (Audio|SpawnSound2D "/Game/Music/SoundCues/SFX/SQ_Ice.SQ_Ice" 1.0 1.0 0.0 0))
  (Collision|SetCollisionResponsetoChannel _cube "ECC_Pawn" "ECR_Overlap")
  (Rendering|Material|SetMaterial _cube 0 "/Game/Objects/Weapon/Art/3D/Metall.Metall"))

(fn SwitchtoHotState
  (params (shouldplaySound :type Boolean))
  (bind _cube (Variables|Default|GetCube))
  (if shouldplaySound
    (Audio|SpawnSound2D "/Game/Music/SoundCues/SFX/SQ_Fire.SQ_Fire" 1.0 1.0 0.0 0))
  (Collision|SetCollisionResponsetoChannel _cube "ECC_Pawn" "ECR_Block")
  (Rendering|Material|SetMaterial _cube 0 "/Game/Objects/Weapon/Art/3D/Roth.Roth"))

(fn MakePlayerPerformHighJump
  (params (Target :type BP%20Player%20Object%20Reference))
  (if (Utilities|Enum|Equal(Enum) (Variables|Default|GetHeat%20State) "NewEnumerator15")
    (Default|PerformHighJump Target (Variables|Default|GetJumpVelocity))))

(fn CanPlayerSlide)