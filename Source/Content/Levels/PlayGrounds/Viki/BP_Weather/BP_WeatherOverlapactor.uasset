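; Box trigger actor for weather zones, built to hand its WeatherData to an overlapping BP_WeatherSpawner and clear it on exit.
; HandleOverlap sets the data and IsActive on start, or clears it by key on stop.
; End overlap calls it when active.
; Begin overlap only loads and casts the save slot; the isWeatherOn check that would apply weather is disconnected, so entry applies nothing.
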(event OnComponentEndOverlap(Box)
  (params (OverlappedComponent :type Primitive%20Component%20Object%20Reference) (OtherActor :type Actor%20Object%20Reference) (OtherComp :type Primitive%20Component%20Object%20Reference) (OtherBodyIndex :type Integer))
  (if (Variables|Default|GetIsActive)
    (CallFunction|HandleOverlap (Variables|Default|GetOnEndOverlap) OtherActor)))

(event OnComponentBeginOverlap(Box)
  (params (OverlappedComponent :type Primitive%20Component%20Object%20Reference) (OtherActor :type Actor%20Object%20Reference) (OtherComp :type Primitive%20Component%20Object%20Reference) (OtherBodyIndex :type Integer) (bFromSweep :type Boolean) (SweepResult :type Hit%20Result%20Structure%20%28by%20ref%29))
  (bind _returnvalue (SaveGame|DoesSaveGameExist "MyCoolSlot"))
  (if _returnvalue
    (bind _returnvalue_2 (SaveGame|LoadGamefromSlot "MyCoolSlot"))
    (bind _asbp_save_game_save_slot_one (Utilities|Casting|CastToBP_SaveGame_SaveSlotOne _returnvalue_2))))

(fn ConstructionScript)

(fn HandleOverlap
  (params (OverlapType :type OverlapType%20Enum :default "NewEnumerator0") (OtherActor :type Actor%20Object%20Reference))
  (bind _asbp_weather_spawner (Utilities|Casting|CastToBP_WeatherSpawner OtherActor))
  (switch Utilities|FlowControl|Switch|SwitchonOverlapType OverlapType
    (:NewEnumerator1
      (Default|SetWeatherData _asbp_weather_spawner (Variables|Default|GetWeatherData))
      (Variables|Default|SetIsActive true))
    (:NewEnumerator2
      (Default|ClearWethaerData _asbp_weather_spawner (.key (Variables|Default|GetWeatherData))))))