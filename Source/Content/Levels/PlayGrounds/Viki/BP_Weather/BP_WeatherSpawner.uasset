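; Weather spawner actor that follows the player and plays the active weather's Niagara effect and sound.
; SetWeatherData ignores an already-active key, otherwise applies the particle asset and amount, fades in audio and stores follow speed.
; ClearWethaerData deactivates the effect and fades out audio when the key matches.
; Tick interpolates from the player pawn's location, not its own, toward the player character, so follow speed normally adds no lag.
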(event EventBeginPlay
  (Variables|Default|SetActorToFollow (Game|GetPlayerCharacter 0)))

(event Collision|EventActorBeginOverlap
  (params (OtherActor :type Actor%20Object%20Reference)))

(event EventTick
  (params (DeltaSeconds :type Float%20%28single-precision%29))
  (bind _actortofollow (Variables|Default|GetActorToFollow))
  (if (Utilities|IsValid _actortofollow)
    (Transformation|SetActorLocation (Math|Interpolation|VInterpTo (Transformation|GetActorLocation (Game|Player|GetPlayerPawn 0)) (Transformation|GetActorLocation _actortofollow) DeltaSeconds (Variables|Default|GetFollowingSpeed)) false false)))

(fn ConstructionScript)

(fn SetWeatherData
  (params (WeatherData :type F%20Weather%20Data%20Structure))
  (bind _niagara (Variables|Default|GetNiagara))
  (bind _niagara_2 (Variables|Default|GetNiagara))
  (bind _audio (Variables|Default|GetAudio))
  (if (== (Variables|Default|GetCurrentKey) (.key WeatherData))
    (return)
    (else
      (Variables|Default|SetCurrentKey (.key WeatherData))
      (Utilities|FlowControl|Sequence
        (:then_0
          ;[0.000493 0 0.01562] Particle System
          (if (Utilities|IsValid (.particlesystem WeatherData))
            (if (Components|Activation|IsActive _niagara)
              _
              (else
                (Components|Activation|Activate _niagara false)))
            (Class|NiagaraComponent|SetAsset _niagara_2 (.particlesystem WeatherData) true)
            (Niagara|SetNiagaraVariable(Float) _niagara_2 "Amount" (.amount WeatherData))
            (Development|PrintString "particle")))
        (:then_1
          ;[0.000304 0 0.006049] Sound
          (if (Utilities|IsValid (.sound WeatherData))
            (Audio|Components|Audio|SetSound _audio (.sound WeatherData))
            (Audio|Components|Audio|FadeIn _audio 1.0 1.0 0.0 "Linear" :!class /Script/Engine.AudioComponent)
            (Development|PrintString "sound")))
        (:then_2
          ;[0.000304 0 0.006049] Following Speed
          (Variables|Default|SetFollowingSpeed (.followingspeed WeatherData)))))))

(fn ClearWethaerData
  (params (Key :type Name))
  (if (== Key (Variables|Default|GetCurrentKey))
    (Variables|Default|SetCurrentKey "None")
    (Components|Activation|Deactivate (Variables|Default|GetNiagara))
    (Variables|Default|SetFollowingSpeed 1.0)
    (Audio|Components|Audio|FadeOut (Variables|Default|GetAudio) 1.0 0.0 "Linear" :!class /Script/Engine.AudioComponent)))