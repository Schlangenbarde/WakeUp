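; BP_Bayblade is a spinning object that carries four Umbrella actors around with it.
; At BeginPlay, a Rotation variable sets the single-axis rate of its RotatingMovement component.
; Every tick, it teleport-free and sweep-free snaps each Umbrella to the world location of its matching ChildActor component.
; Only location is copied, so the umbrellas follow the spinning anchor points without inheriting their rotation from this Blueprint.
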(event EventBeginPlay
  (Variables|/Script/Engine.RotatingMovementComponent|SetRotationRate (Variables|Default|GetRotatingMovement) (Math|Rotator|MakeRotator 0.0 0.0 (Variables|Default|GetRotation))))

(event EventTick
  (params (DeltaSeconds :type Float%20%28single-precision%29))
  (Transformation|SetActorLocation (Variables|Default|GetUmbrella) (Transformation|GetWorldLocation (Variables|Default|GetChildActor)) false false)
  (Transformation|SetActorLocation (Variables|Default|GetUmbrella_1) (Transformation|GetWorldLocation (Variables|Default|GetChildActor1)) false false)
  (Transformation|SetActorLocation (Variables|Default|GetUmbrella_2) (Transformation|GetWorldLocation (Variables|Default|GetChildActor2)) false false)
  (Transformation|SetActorLocation (Variables|Default|GetUmbrella_3) (Transformation|GetWorldLocation (Variables|Default|GetChildActor3)) false false))

(fn ConstructionScript)