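; BP_WIN is a win-celebration actor that stays inert until the referenced collection reports all collectables collected.
; It binds to that collection's OnAllCollected event on BeginPlay, which arms its overlap trigger.
; When the player then overlaps the trigger, it plays a win animation and spawns confetti and fireworks Niagara effects at four child-actor locations.
; After a short delay it destroys itself, spawning a final confetti burst.
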(event OnComponentBeginOverlap(ActivateCollision)
  (params (OverlappedComponent :type Primitive%20Component%20Object%20Reference) (OtherActor :type Actor%20Object%20Reference) (OtherComp :type Primitive%20Component%20Object%20Reference) (OtherBodyIndex :type Integer) (bFromSweep :type Boolean) (SweepResult :type Hit%20Result%20Structure%20%28by%20ref%29))
  (Utilities|Casting|CastToBP_Player OtherActor)
  (if (Variables|Default|GetCanActivate)
    (Audio|Components|Audio|Play (Variables|Default|GetWin_Anim_) false)
    (Niagara|SpawnSystematLocation "/Game/Levels/PlayGrounds/Chiara/VFX/NS_Confetti.NS_Confetti" (Transformation|GetWorldLocation (Variables|Default|GetChildActor)))
    (Niagara|SpawnSystematLocation "/Game/Levels/PlayGrounds/Chiara/Firework/NS_Fireworks.NS_Fireworks" (Transformation|GetWorldLocation (Variables|Default|GetChildActor1)))
    (Niagara|SpawnSystematLocation "/Game/Levels/PlayGrounds/Chiara/VFX/NS_Confetti.NS_Confetti" (Transformation|GetWorldLocation (Variables|Default|GetChildActor2)))
    (Niagara|SpawnSystematLocation "/Game/Levels/PlayGrounds/Chiara/Firework/NS_Fireworks.NS_Fireworks" (Transformation|GetWorldLocation (Variables|Default|GetChildActor3)))
    (Utilities|FlowControl|Delay 2.0)
    (Actor|DestroyActor)))

(event Custom|OnAllCollected
  (Variables|Default|SetCanActivate true))

(event EventDestroyed
  (Niagara|SpawnSystematLocation "/Game/Levels/PlayGrounds/Chiara/VFX/NS_Confetti.NS_Confetti" (Transformation|GetActorLocation)))

(event EventBeginPlay
  (EventDispatchers|BindEventtoOnAllCollected (Variables|Default|GetCollectionofCollectables) (EventDispatchers|CreateEvent :!event Custom|OnAllCollected)))

(fn ConstructionScript)