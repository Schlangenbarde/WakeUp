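; Interactable wall platform that switches between a solid cold state and a passable hot state.
; Cold swaps Cube to an ice mesh and material, blocks Pawns and destroys any stored VFX.
; Hot swaps to the box look, ignores Pawns and spawns a particle system sized from marker component distances and rotated by root yaw.
; Both switches can optionally play an ice or fire sound.
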(fn ConstructionScript
  (|CallParentFunction))

(fn SwitchtoColdState
  (params (shouldplaySound :type Boolean))
  (bind _cube (Variables|Default|GetCube))
  (bind _vfx (Variables|Default|GetVFX))
  (if shouldplaySound
    (Audio|SpawnSound2D "/Game/Music/SoundCues/SFX/SQ_Ice.SQ_Ice" 1.0 1.0 0.0 0))
  (Rendering|Material|SetMaterial _cube 0 "/Game/Levels/PlayGrounds/Kathleen/Material/Mat_IceShader/MAT_TestICE_02_Inst.MAT_TestICE_02_Inst")
  (Collision|SetCollisionResponsetoChannel _cube "ECC_Pawn" "ECR_Block")
  (Components|StaticMesh|SetStaticMesh _cube "/Game/Objects/Plattforms/Meshes/OBJ_BeveledSquare5x1x5ICE_002.OBJ_BeveledSquare5x1x5ICE_002")
  (if (Utilities|IsValid _vfx)
    (Components|DestroyComponent _vfx)))

(fn SwitchtoHotState
  (params (shouldplaySound :type Boolean))
  (bind _cube (Variables|Default|GetCube))
  (if shouldplaySound
    (Audio|SpawnSound2D "/Game/Music/SoundCues/SFX/SQ_Fire.SQ_Fire" 1.0 1.0 0.0 0))
  (Rendering|Material|SetMaterial _cube 0 "/Game/Levels/PlayGrounds/Chiara/MAT_Box.MAT_Box")
  (Collision|SetCollisionResponsetoChannel _cube "ECC_Pawn" "ECR_Ignore")
  (Components|StaticMesh|SetStaticMesh _cube "/Game/Objects/Plattforms/Meshes/OBJ_BeveledSquare5x1x5_001.OBJ_BeveledSquare5x1x5_001")
  (bind _returnvalue (Niagara|SpawnSystematLocation (Variables|Default|GetSystem%20Template) (Transformation|GetWorldLocation (Variables|Default|GetChildActor)) "0, 0, 0" "1.000000,1.000000,1.000000" false false))
  (Variables|Default|SetVFX _returnvalue)
  (Effects|Components|ParticleSystem|SetVectorParameter _returnvalue "User.Length" (Math|Vector|MakeVector (Math|Vector|Distance(Vector) (Transformation|GetWorldLocation (Variables|Default|GetTop)) (Transformation|GetWorldLocation (Variables|Default|GetChildActor3))) (Math|Vector|Distance(Vector) (Transformation|GetWorldLocation (Variables|Default|GetChildActor3)) (Transformation|GetWorldLocation (Variables|Default|GetChildActor2))) 0.0))
  (Effects|Components|ParticleSystem|SetVectorParameter _returnvalue "User.Rotation" (Math|Vector|MakeVector (.yaw (Transformation|GetWorldRotation (Variables|Default|GetDefaultSceneRoot))) 0.0 0.0))
  (Components|Activation|Activate _returnvalue false))