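; Moving platform that shuttles between two placed reference actors, PositionOne and PositionTwo.
; Tick steps it toward the target by Speed per frame without delta-time scaling, snaps on arrival, then alternates targets through a Delay and FlipFlop.
; Move switches ticking and motion, spawning or destroying the attached flight sound.
; Nitro spawns particle effects at four scene points, but its event-graph call is disconnected.
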(event EventBeginPlay
  (Variables|Default|SetTarget (Transformation|GetActorLocation (Variables|Default|GetPositionOne)))
  (Components|StaticMesh|SetStaticMesh (Variables|Default|GetCube) 0))

(event EventTick
  (params (DeltaSeconds :type Float%20%28single-precision%29))
  (if (Variables|Default|GetisMoving)
    (if (<= (Math|Vector|Distance(Vector) (Variables|Default|GetTarget) (Transformation|GetActorLocation)) (Variables|Default|GetSpeed))
      (Transformation|SetActorLocation (Variables|Default|GetTarget) false false)
      (Utilities|FlowControl|Delay (Variables|Default|GetWaitTimer))
      (Utilities|FlowControl|FlipFlop
        (:A
          (Variables|Default|SetTarget (Transformation|GetActorLocation (Variables|Default|GetPositionOne))))
        (:B
          (Variables|Default|SetTarget (Transformation|GetActorLocation (Variables|Default|GetPositionTwo)))))
      (else
        (Transformation|SetActorLocation (+ (* (Math|Vector|Normalize (- (Variables|Default|GetTarget) (Transformation|GetActorLocation))) (Variables|Default|GetSpeed)) (Transformation|GetActorLocation)) false false)))))

(fn ConstructionScript)

(fn Move
  (params (isMoving :type Boolean))
  (Actor|Tick|SetActorTickEnabled isMoving)
  (bind _output_get (Variables|Default|SetisMoving isMoving))
  (if _output_get
    (bind _returnvalue (Audio|SpawnSoundAttached "/Game/Music/SoundCues/Special/Fly.Fly" (Variables|Default|GetBox) "None" "0, 0, 0" "0, 0, 0" "KeepRelativeOffset" false 1.0 1.0 0.0 0 0))
    (Variables|Default|SetSound _returnvalue)
    (else
      (Utilities|IsValid (Variables|Default|GetSound)
        (:Is%20Valid
          (Audio|Components|Audio|Stop (Variables|Default|GetSound))
          (Components|DestroyComponent (Variables|Default|GetSound)))))))

(fn Nitro
  (Niagara|SpawnSystematLocation "/Game/Levels/PlayGrounds/Chiara/VFX/Nitro.Nitro" (Transformation|GetWorldLocation (Variables|Default|GetScene)) "0.000000,0.000000,180.000000" "0.100000,0.100000,0.100000")
  (Niagara|SpawnSystematLocation "/Game/Levels/PlayGrounds/Chiara/VFX/Nitro.Nitro" (Transformation|GetWorldLocation (Variables|Default|GetScene1)) "0.000000,0.000000,180.000000" "0.100000,0.100000,1.000000")
  (Niagara|SpawnSystematLocation "/Game/Levels/PlayGrounds/Chiara/VFX/Nitro.Nitro" (Transformation|GetWorldLocation (Variables|Default|GetScene2)) "0.000000,0.000000,180.000000" "0.100000,0.100000,0.100000")
  (Niagara|SpawnSystematLocation "/Game/Levels/PlayGrounds/Chiara/VFX/Nitro.Nitro" (Transformation|GetWorldLocation (Variables|Default|GetScene3)) "0.000000,0.000000,180.000000" "0.100000,0.100000,0.100000"))