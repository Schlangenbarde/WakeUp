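; Interactable that controls a flying platform by switching between cold and hot states.
; The hot state calls Move(true) on the referenced platform, plays fire and loading sounds if requested, hides a static mesh and plays a one-shot capsule animation.
; The cold state calls Move(false), plays an optional ice sound and shows the mesh again.
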(fn ConstructionScript
  (|CallParentFunction))

(fn SwitchtoColdState
  (params (shouldplaySound :type Boolean))
  (if shouldplaySound
    (Audio|SpawnSound2D "/Game/Music/SoundCues/SFX/SQ_Ice.SQ_Ice" 1.0 1.0 0.0 0))
  (Default|Move (Variables|Default|GetAs%20BP%20Flying%20Plattform) false)
  (CallFunction|ToggleObject true))

(fn SwitchtoHotState
  (params (shouldplaySound :type Boolean))
  (if shouldplaySound
    (Audio|SpawnSound2D "/Game/Music/SoundCues/SFX/SQ_Fire.SQ_Fire" 1.0 1.0 0.0 0)
    (Audio|SpawnSound2D "/Game/Music/SoundCues/Special/Loading.Loading" 1.0 1.0 0.0 0))
  (Default|Move (Variables|Default|GetAs%20BP%20Flying%20Plattform) true)
  (CallFunction|ToggleObject false)
  (Components|Animation|PlayAnimation (Variables|Default|Getcapsule_02) "/Game/Objects/Switch/Mesh/capsule_02_Anim.capsule_02_Anim" false))

(fn ToggleObject
  (params (coldIsActive :type Boolean))
  (Rendering|SetVisibility (Variables|Default|GetStaticMesh) coldIsActive false))