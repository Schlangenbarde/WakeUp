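; Umbrella jump pad interactable that switches between hot and cold states, launching BP_Player into a high jump in one heat state.
; State switches swap meshes, visibility, collision responses and idle bob height, with optional sound.
; Hot is a bobbing cloth umbrella whose box blocks normal jumping; cold is a still ice umbrella that triggers the player's frozen-ground behavior.
; Mesh hits and overlap exits request the launch, gated by HeatState.
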(event OnComponentBeginOverlap(Box)
  (params (OverlappedComponent :type Primitive%20Component%20Object%20Reference) (OtherActor :type Actor%20Object%20Reference) (OtherComp :type Primitive%20Component%20Object%20Reference) (OtherBodyIndex :type Integer) (bFromSweep :type Boolean) (SweepResult :type Hit%20Result%20Structure%20%28by%20ref%29))
  (bind _asbp_player (Utilities|Casting|CastToBP_Player OtherActor))
  (Variables|/Game/Objects/Player/Code/BP_Player.BP_Player_C|SetMyCanJump _asbp_player false))

(event OnComponentEndOverlap(Box)
  (params (OverlappedComponent :type Primitive%20Component%20Object%20Reference) (OtherActor :type Actor%20Object%20Reference) (OtherComp :type Primitive%20Component%20Object%20Reference) (OtherBodyIndex :type Integer))
  (bind _asbp_player (Utilities|Casting|CastToBP_Player OtherActor))
  (Variables|/Game/Objects/Player/Code/BP_Player.BP_Player_C|SetMyCanJump _asbp_player true))

(event OnComponentEndOverlap(StaticMesh)
  (params (OverlappedComponent :type Primitive%20Component%20Object%20Reference) (OtherActor :type Actor%20Object%20Reference) (OtherComp :type Primitive%20Component%20Object%20Reference) (OtherBodyIndex :type Integer))
  (bind _asbp_player (Utilities|Casting|CastToBP_Player OtherActor))
  (Default|PerformUnfrozen _asbp_player)
  (CallFunction|MakePlayerPerformHighJump _asbp_player))

(event OnComponentHit(StaticMesh)
  (params (HitComponent :type Primitive%20Component%20Object%20Reference) (OtherActor :type Actor%20Object%20Reference) (OtherComp :type Primitive%20Component%20Object%20Reference) (NormalImpulse :type Vector :default "0, 0, 0") (Hit :type Hit%20Result%20Structure%20%28by%20ref%29))
  (bind _asbp_player (Utilities|Casting|CastToBP_Player OtherActor))
  (CallFunction|MakePlayerPerformHighJump _asbp_player))

(event OnComponentBeginOverlap(StaticMesh)
  (params (OverlappedComponent :type Primitive%20Component%20Object%20Reference) (OtherActor :type Actor%20Object%20Reference) (OtherComp :type Primitive%20Component%20Object%20Reference) (OtherBodyIndex :type Integer) (bFromSweep :type Boolean) (SweepResult :type Hit%20Result%20Structure%20%28by%20ref%29))
  (bind _asbp_player (Utilities|Casting|CastToBP_Player OtherActor))
  (Default|PerformFrozenGround _asbp_player))

(event Custom|IdleMovement
  (bind _returnvalue (Transformation|GetActorLocation))
  ;[1 1 1] Idle Movement
  (bind _movementtrack (Timeline|Timeline Play)
    (:Update
      (Transformation|SetWorldLocation (Variables|Default|GetStaticMesh) (Math|Vector|Lerp(Vector) (+ _returnvalue (Math|Vector|MakeVector 0.0 0.0 (Variables|Default|GetZ%20Movement))) _returnvalue _movementtrack) false false))))

(event EventBeginPlay
  (|CallParentFunction)
  (Variables|Default|SetStartingPosition (Transformation|GetWorldLocation (Variables|Default|GetStaticMesh)))
  (CallFunction|IdleMovement))

(fn ConstructionScript
  (|CallParentFunction))

(fn Interact
  (params (incomingHeat :type ENUM_HeatState%20Enum :default "NewEnumerator13"))
  (|CallParentFunction incomingHeat))

(fn SwitchtoColdState
  (params (shouldplaySound :type Boolean))
  (if shouldplaySound
    (Audio|SpawnSound2D "/Game/Music/SoundCues/SFX/SQ_Ice.SQ_Ice" 1.0 1.0 0.0 0))
  (Components|StaticMesh|SetStaticMesh (Variables|Default|GetStaticMesh) "/Game/Objects/Interactable/JumpPad/Art/3DMesh/OBJ_Umbrella_ICE_006.OBJ_Umbrella_ICE_006")
  (Collision|SetCollisionResponsetoChannel (Variables|Default|GetStaticMesh) "ECC_Pawn" "ECR_Overlap")
  (Collision|SetCollisionResponsetoChannel (Variables|Default|GetIceCollision) "ECC_Pawn" "ECR_Block")
  (Collision|SetCollisionResponsetoChannel (Variables|Default|GetBox) "ECC_Pawn" "ECR_Ignore")
  (Rendering|SetVisibility (Variables|Default|GetStaticMesh) true false)
  (Rendering|SetVisibility (Variables|Default|GetCloth_Umbrella) false false)
  (Rendering|SetVisibility (Variables|Default|GetOBJ_Umbrella_Base_Animation_004) false false)
  (Variables|Default|SetZ%20Movement 0.0))

(fn SwitchtoHotState
  (params (shouldplaySound :type Boolean))
  (bind _mattest (Variables|Default|GetMatTest))
  (if shouldplaySound
    (Audio|SpawnSound2D "/Game/Music/SoundCues/SFX/SQ_Fire.SQ_Fire" 1.0 1.0 0.0 0))
  (Components|StaticMesh|SetStaticMesh (Variables|Default|GetStaticMesh) "/Game/Objects/Interactable/JumpPad/Art/3DMesh/OBJ_Umbrella_023.OBJ_Umbrella_023")
  (Utilities|IsValid _mattest
    (:Is%20Valid
      (Rendering|Material|SetMaterial (Variables|Default|GetCloth_Umbrella) 0 _mattest))
    (:Is%20Not%20Valid
      _))
  (Collision|SetCollisionResponsetoChannel (Variables|Default|GetStaticMesh) "ECC_Pawn" "ECR_Block")
  (Collision|SetCollisionResponsetoAllChannels (Variables|Default|GetIceCollision) "ECR_Ignore")
  (Collision|SetCollisionResponsetoChannel (Variables|Default|GetBox) "ECC_Pawn" "ECR_Overlap")
  (Rendering|SetVisibility (Variables|Default|GetStaticMesh) false false)
  (Rendering|SetVisibility (Variables|Default|GetCloth_Umbrella) true false)
  (Rendering|SetVisibility (Variables|Default|GetOBJ_Umbrella_Base_Animation_004) true false)
  (Variables|Default|SetZ%20Movement 2e+01))

(fn MakePlayerPerformHighJump
  (params (Target :type BP%20Player%20Object%20Reference))
  (if (Utilities|Enum|Equal(Enum) (Variables|Default|GetHeat%20State) "NewEnumerator15")
    (Default|PerformHighJump Target (Variables|Default|GetJumpVelocity))
    (Audio|SpawnSound2D "/Game/Music/SoundCues/Special/Jump.Jump" 1.0 1.0 0.0 0)))

(fn CanPlayerSlide)