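; Test jump pad interactable that launches the player with a high jump while its heat state matches one specific value.
; Hit and end-overlap events on the mesh trigger the jump, while begin and end overlap also toggle the player's frozen-ground behavior.
; Hot and cold switches play a sound and swap Pawn blocking between the main mesh and ice collision.
; A timeline bobs the mesh vertically from its start position.
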(event OnComponentEndOverlap(StaticMesh)
  (params (OverlappedComponent :type Primitive%20Component%20Object%20Reference) (OtherActor :type Actor%20Object%20Reference) (OtherComp :type Primitive%20Component%20Object%20Reference) (OtherBodyIndex :type Integer))
  (bind _asbp_player (Utilities|Casting|CastToBP_Player OtherActor))
  (Default|PerformUnfrozen _asbp_player)
  (CallFunction|MakePlayerPerformHighJump _asbp_player))

(event OnComponentHit(StaticMesh)
  (params (HitComponent :type Primitive%20Component%20Object%20Reference) (OtherActor :type Actor%20Object%20Reference) (OtherComp :type Primitive%20Component%20Object%20Reference) (NormalImpulse :type Vector :default "0, 0, 0") (Hit :type Hit%20Result%20Structure%20%28by%20ref%29))
  (bind _asbp_player (Utilities|Casting|CastToBP_Player OtherActor))
  (CallFunction|MakePlayerPerformHighJump _asbp_player))

(event OnComponentBeginOverlap(StaticMesh)
  (params (OverlappedComponent :type Primitive%20Component%20Object%20Reference) (OtherActor :type Actor%20Object%20Reference) (OtherComp :type Primitive%20Component%20Object%20Reference) (OtherBodyIndex :type Integer) (bFromSweep :type Boolean) (SweepResult :type Hit%20Result%20Structure%20%28by%20ref%29))
  (bind _asbp_player (Utilities|Casting|CastToBP_Player OtherActor))
  (Default|PerformFrozenGround _asbp_player))

(event Custom|IdleMovement
  (bind _startingposition (Variables|Default|GetStartingPosition))
  ;[1 1 1] Idle Movement
  (bind _movementtrack (Timeline|Bounce PlayFromStart)
    (:Update
      (Transformation|SetWorldLocation (Variables|Default|GetStaticMesh) (Math|Vector|Lerp(Vector) (+ _startingposition (Math|Vector|MakeVector 0.0 0.0 (Variables|Default|Getz%20Movement))) _startingposition _movementtrack) false false))))

(event EventBeginPlay
  (Variables|Default|SetStartingPosition (Transformation|GetWorldLocation (Variables|Default|GetStaticMesh)))
  (CallFunction|IdleMovement))

(fn ConstructionScript
  (|CallParentFunction))

(fn Interact
  (params (incomingHeat :type ENUM_HeatState%20Enum :default "NewEnumerator13"))
  (|CallParentFunction incomingHeat))

(fn SwitchtoColdState
  (Audio|SpawnSound2D "/Game/Music/SoundCues/SFX/SQ_Ice.SQ_Ice" 1.0 1.0 0.0 0)
  (Collision|SetCollisionResponsetoChannel (Variables|Default|GetStaticMesh) "ECC_Pawn" "ECR_Overlap")
  (Collision|SetCollisionResponsetoChannel (Variables|Default|GetIceCollision) "ECC_Pawn" "ECR_Block"))

(fn SwitchtoHotState
  (Audio|SpawnSound2D "/Game/Music/SoundCues/SFX/SQ_Fire.SQ_Fire" 1.0 1.0 0.0 0)
  (Collision|SetCollisionResponsetoChannel (Variables|Default|GetStaticMesh) "ECC_Pawn" "ECR_Block")
  (Collision|SetCollisionResponsetoAllChannels (Variables|Default|GetIceCollision) "ECR_Ignore"))

(fn MakePlayerPerformHighJump
  (params (Target :type BP%20Player%20Object%20Reference))
  (if (Utilities|Enum|Equal(Enum) (Variables|Default|GetHeat%20State) "NewEnumerator15")
    (Default|PerformHighJump Target (Variables|Default|GetJumpVelocity))))

(fn CanPlayerSlide)