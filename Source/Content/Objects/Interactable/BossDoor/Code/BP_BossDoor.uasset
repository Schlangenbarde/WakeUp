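; BP_BossDoor is a level-exit door that stays locked until its bound collectables collection reports all collected.
; That event swaps the closed door for the open one, enables the trigger box and spawns a light effect at the child actor.
; A player overlapping the box loads LevelToLoad behind a loading screen widget.
; Once unlocked, LightCollision removes the effect while the player is inside and respawns it on exit.
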(event OnComponentBeginOverlap(Box)
  (params (OverlappedComponent :type Primitive%20Component%20Object%20Reference) (OtherActor :type Actor%20Object%20Reference) (OtherComp :type Primitive%20Component%20Object%20Reference) (OtherBodyIndex :type Integer) (bFromSweep :type Boolean) (SweepResult :type Hit%20Result%20Structure%20%28by%20ref%29))
  (Utilities|Casting|CastToBP_Player OtherActor)
  (Viewport|RemoveAllWidgets)
  (Game|OpenLevel(byObjectReference) (Variables|Default|GetLevelToLoad))
  (bind _returnvalue (UserInterface|CreateWidget "/Game/Art/2D/UI/Prototyp_Screens/WBP_LoadingScreen.WBP_LoadingScreen_C"))
  (UserInterface|Viewport|AddtoViewport _returnvalue 0))

(event OnComponentBeginOverlap(LightCollision)
  (params (OverlappedComponent :type Primitive%20Component%20Object%20Reference) (OtherActor :type Actor%20Object%20Reference) (OtherComp :type Primitive%20Component%20Object%20Reference) (OtherBodyIndex :type Integer) (bFromSweep :type Boolean) (SweepResult :type Hit%20Result%20Structure%20%28by%20ref%29))
  (Utilities|Casting|CastToBP_Player OtherActor)
  (if (and (Utilities|IsValid (Variables|Default|GetVFX)) (Variables|Default|GetisInteractable))
    (Components|DestroyComponent (Variables|Default|GetVFX))))

(event OnComponentEndOverlap(LightCollision)
  (params (OverlappedComponent :type Primitive%20Component%20Object%20Reference) (OtherActor :type Actor%20Object%20Reference) (OtherComp :type Primitive%20Component%20Object%20Reference) (OtherBodyIndex :type Integer))
  (Utilities|Casting|CastToBP_Player OtherActor)
  (if (and (not (Utilities|IsValid (Variables|Default|GetVFX))) (Variables|Default|GetisInteractable))
    (bind _returnvalue (Niagara|SpawnSystematLocation "/Game/Levels/PlayGrounds/Chiara/VFX/Infinite_Light_End.Infinite_Light_End" (Transformation|GetWorldLocation (Variables|Default|GetChildActor)) "0, 0, 0" "1.000000,1.000000,1.000000" false))
    (Variables|Default|SetVFX _returnvalue)))

(event Custom|OnAllCollected
  (Variables|Default|SetisInteractable true)
  (Collision|SetCollisionEnabled (Variables|Default|GetBox) "QueryAndPhysics")
  (Rendering|SetVisibility (Variables|Default|GetDoorClosed) false true)
  (Rendering|SetVisibility (Variables|Default|GetDoorOpen) true true)
  (bind _returnvalue (Niagara|SpawnSystematLocation "/Game/Levels/PlayGrounds/Chiara/VFX/Infinite_Light_End.Infinite_Light_End" (Transformation|GetWorldLocation (Variables|Default|GetChildActor)) "0, 0, 0" "1.000000,1.000000,1.000000" false))
  (Variables|Default|SetVFX _returnvalue))

(event EventBeginPlay
  (EventDispatchers|BindEventtoOnAllCollected (Variables|Default|GetCollectionOfCollecteables) (EventDispatchers|CreateEvent :!event Custom|OnAllCollected))
  (Rendering|SetVisibility (Variables|Default|GetDoorOpen) false true)
  (Components|StaticMesh|SetStaticMesh (Variables|Default|GetDoor) 0))

(fn ConstructionScript)