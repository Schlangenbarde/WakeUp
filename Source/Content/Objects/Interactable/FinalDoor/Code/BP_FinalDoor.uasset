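; Boss door that opens when its collectible set is complete, with a trigger box that sends the player to another level.
; While locked, inner and outer proximity circles step the light intensity, and the inner one layers two music tracks; outer-circle music is disabled.
; Collecting all plays a montage and sound, hides the door and removes collision.
; Box overlap swaps the skybox, spawns particles and loads the level.
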(event OnComponentBeginOverlap(Box)
  (params (OverlappedComponent :type Primitive%20Component%20Object%20Reference) (OtherActor :type Actor%20Object%20Reference) (OtherComp :type Primitive%20Component%20Object%20Reference) (OtherBodyIndex :type Integer) (bFromSweep :type Boolean) (SweepResult :type Hit%20Result%20Structure%20%28by%20ref%29))
  (bind _sm_skybox (Variables|Default|GetSM_Skybox))
  (bind _staticmeshcomponent (Variables|/Script/Engine.StaticMeshActor|GetStaticMeshComponent _sm_skybox))
  (Utilities|Casting|CastToBP_Player OtherActor)
  (Components|StaticMesh|SetStaticMesh _staticmeshcomponent (Variables|Default|GetMeshAfterPlayerEntered))
  (Rendering|Material|SetMaterial _staticmeshcomponent 0 (Variables|Default|GetMaterialAfterPlayerEntered))
  (Effects|SpawnEmitteratLocation 0 (Transformation|GetActorLocation OtherActor))
  (Game|OpenLevel(byObjectReference) (Variables|Default|GetLevelToLoad)))

(event Custom|OnEnterInnerCircle
  (CallFunction|SetLightIntensity 4e+03)
  (if (not (Variables|Default|GetisInteractable))
    (bind _returnvalue (Audio|SpawnSound2D "/Game/Music/SoundCues/SFX/SC_MoreIntenceMusic.SC_MoreIntenceMusic" 1.0 1.0 0.0 0))
    (Variables|Default|SetMoreIntenseMusic _returnvalue)
    (bind _returnvalue_2 (Audio|SpawnSound2D "/Game/Music/SoundCues/SFX/SC_IntenceMusic.SC_IntenceMusic" 1.0 1.0 0.0 0))
    (Variables|Default|SetIntenseMusic _returnvalue_2)))

(event Custom|OnLeaveInnerCircle
  (bind _moreintensemusic (Variables|Default|GetMoreIntenseMusic))
  (bind _intensemusic (Variables|Default|GetIntenseMusic))
  (CallFunction|SetLightIntensity 2e+03)
  (if (Utilities|IsValid _intensemusic)
    (Components|DestroyComponent _intensemusic)
    (if (Utilities|IsValid _moreintensemusic)
      (Components|DestroyComponent _moreintensemusic))))

(event Custom|OnEnterOuterCircle
  (if (not true)
    (CallFunction|SetLightIntensity 2e+03)
    (bind _returnvalue (Audio|SpawnSound2D "/Game/Music/SoundCues/SFX/SC_IntenceMusic.SC_IntenceMusic" 1.0 1.0 0.0 0))
    (Variables|Default|SetIntenseMusic _returnvalue)))

(event Custom|OnLeaveOuterCircle
  (bind _intensemusic (Variables|Default|GetIntenseMusic))
  (CallFunction|SetLightIntensity 1e+03)
  (if (Utilities|IsValid _intensemusic)
    (Components|DestroyComponent _intensemusic)))

(event Custom|OnAllCollected
  (bind _door (Variables|Default|GetDoor))
  (Development|PrintString "Boss Door open")
  (Variables|Default|SetisInteractable true)
  (Animation|Montage|PlayMontage (Variables|Default|GetSkeletalMesh) 0
    (:then
      (Audio|PlaySoundatLocation "/Game/Music/SoundCues/SFX/SC_BossDoorOpen.SC_BossDoorOpen" (Transformation|GetWorldLocation (Variables|Default|GetDoor)) "0, 0, 0" 1.0 1.0 0.0 0 0 0 0)
      (Rendering|SetVisibility _door false false)
      (Collision|SetCollisionResponsetoAllChannels _door "ECR_Ignore"))))

(event EventBeginPlay
  (bind _twostepinteractable (Variables|Default|GettwoStepInteractable))
  (EventDispatchers|BindEventtoOnEnterInnerCircle _twostepinteractable (EventDispatchers|CreateEvent :!event Custom|OnEnterInnerCircle))
  (EventDispatchers|BindEventtoOnLeaveInnerCircle _twostepinteractable (EventDispatchers|CreateEvent :!event Custom|OnLeaveInnerCircle))
  (EventDispatchers|BindEventtoOnEnterOuterCircle _twostepinteractable (EventDispatchers|CreateEvent :!event Custom|OnEnterOuterCircle))
  (EventDispatchers|BindEventtoOnLeaveOuterCircle _twostepinteractable (EventDispatchers|CreateEvent :!event Custom|OnLeaveOuterCircle))
  (EventDispatchers|BindEventtoOnAllCollected (Variables|Default|GetCollectionOfCollecteables) (EventDispatchers|CreateEvent :!event Custom|OnAllCollected)))

(fn ConstructionScript)

(fn SetLightIntensity
  (params (Value :type Float%20%28single-precision%29))
  (if (not (Variables|Default|GetisInteractable))
    (Rendering|Components|Light|SetIntensity (Variables|Default|GetPointLight) Value)
    (Rendering|Components|Light|SetIntensity (Variables|Default|GetPointLight3) Value)
    (Rendering|Components|Light|SetIntensity (Variables|Default|GetPointLight1) Value)
    (Rendering|Components|Light|SetIntensity (Variables|Default|GetPointLight2) Value)))