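; BP_TwoStepsInteractable is an interactable with an outer and an inner trigger zone that reacts to BP_Player with sounds and dispatcher calls on enter and leave.
; The outer zone plays a 2D sound that stops on exit, while the inner zone plays a located sound only on first entry.
; An all-collected callback from CollectionofCollectables suppresses both sounds, and also the inner-enter dispatch if that zone was never entered before.
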(event OnComponentBeginOverlap(Sphere)
  (params (OverlappedComponent :type Primitive%20Component%20Object%20Reference) (OtherActor :type Actor%20Object%20Reference) (OtherComp :type Primitive%20Component%20Object%20Reference) (OtherBodyIndex :type Integer) (bFromSweep :type Boolean) (SweepResult :type Hit%20Result%20Structure%20%28by%20ref%29))
  (Utilities|Casting|CastToBP_Player OtherActor)
  (CallFunction|EnterInnerCircle))

(event OnComponentBeginOverlap(OuterCollistion)
  (params (OverlappedComponent :type Primitive%20Component%20Object%20Reference) (OtherActor :type Actor%20Object%20Reference) (OtherComp :type Primitive%20Component%20Object%20Reference) (OtherBodyIndex :type Integer) (bFromSweep :type Boolean) (SweepResult :type Hit%20Result%20Structure%20%28by%20ref%29))
  (Utilities|Casting|CastToBP_Player OtherActor)
  (CallFunction|EnterOuterCircle))

(event OnComponentEndOverlap(Sphere)
  (params (OverlappedComponent :type Primitive%20Component%20Object%20Reference) (OtherActor :type Actor%20Object%20Reference) (OtherComp :type Primitive%20Component%20Object%20Reference) (OtherBodyIndex :type Integer))
  (Utilities|Casting|CastToBP_Player OtherActor)
  (CallFunction|LeaveInnerCircle))

(event OnComponentEndOverlap(OuterCollistion)
  (params (OverlappedComponent :type Primitive%20Component%20Object%20Reference) (OtherActor :type Actor%20Object%20Reference) (OtherComp :type Primitive%20Component%20Object%20Reference) (OtherBodyIndex :type Integer))
  (Utilities|Casting|CastToBP_Player OtherActor)
  (CallFunction|LeaveOuterCircle))

(event Custom|CustomEvent
  (Variables|Default|SetAllcollected true))

(event EventBeginPlay
  (EventDispatchers|BindEventtoOnAllCollected (Variables|Default|GetcollectionofCollectables) (EventDispatchers|CreateEvent :!event Custom|CustomEvent)))

(fn ConstructionScript)

(fn EnterOuterCircle
  (Default|CallOnEnterOuterCircle)
  (if (not (Variables|Default|GetAllcollected))
    (bind _returnvalue (Audio|SpawnSound2D (Variables|Default|GetoutercircleSound) 1.0 1.0 0.0 0))
    (Variables|Default|SetsavedSound _returnvalue)))

(fn LeaveOuterCircle
  (bind _savedsound (Variables|Default|GetsavedSound))
  (Default|CallOnLeaveOuterCircle)
  (Utilities|IsValid _savedsound
    (:Is%20Valid
      (Audio|Components|Audio|Stop _savedsound)
      (Components|DestroyComponent _savedsound))))

(fn EnterInnerCircle
  (if (Variables|Default|GetAlready%20entered%20inner%20circle)
    (Default|CallOnEnterInnerCircle :!label _label)
    (elif (not (Variables|Default|GetAllcollected))
      (Audio|SpawnSoundatLocation (Variables|Default|GetinnerCircleSound) (Transformation|GetActorLocation) "0, 0, 0" 1.0 1.0 0.0 0 0)
      (Variables|Default|SetAlready%20entered%20inner%20circle true)
      (goto _label))))

(fn LeaveInnerCircle
  (Default|CallOnLeaveInnerCircle))