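; BP_BaseInteractable is a base Blueprint for interactable objects that carry a heat state of cold, normal or hot.
; BeginPlay applies the initial state, passing false for the sound flag on cold and hot.
; Interact takes an incoming heat value, switches only when it differs, requests sound for cold and hot, and prints debug text.
; The three SwitchTo state functions are empty here, apparently left for child classes to override.
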(event EventBeginPlay
  (switch Utilities|FlowControl|Switch|SwitchonENUM_HeatState (Variables|Default|GetHeat%20State)
    (:NewEnumerator13
      (CallFunction|SwitchtoColdState false))
    (:NewEnumerator14
      (CallFunction|SwitchtoNormalState))
    (:NewEnumerator15
      (CallFunction|SwitchtoHotState false))))

(fn ConstructionScript)

(fn Interact
  (params (incomingHeat :type ENUM_HeatState%20Enum :default "NewEnumerator13"))
  (if (Utilities|Enum|NotEqual(Enum) incomingHeat (Variables|Default|GetHeat%20State))
    (bind _output_get (Variables|Default|SetHeat%20State incomingHeat))
    (switch Utilities|FlowControl|Switch|SwitchonENUM_HeatState _output_get
      (:NewEnumerator13
        (CallFunction|SwitchtoColdState true)
        (Development|PrintString "ZUSTAND 0"))
      (:NewEnumerator14
        (CallFunction|SwitchtoNormalState)
        (Development|PrintString "ZUSTAND NORMAl"))
      (:NewEnumerator15
        (CallFunction|SwitchtoHotState true)
        (Development|PrintString "ZUSTAND 2")))
    (else
      (Development|PrintString "The same"))))

(fn SwitchtoColdState
  (params (shouldplaySound :type Boolean)))

(fn SwitchtoNormalState)

(fn SwitchtoHotState
  (params (shouldplaySound :type Boolean)))