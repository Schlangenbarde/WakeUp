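; Interactable moving platform Blueprint that moves a referenced actor between marker actor positions when switched to a cold or hot state.
; Each state switch plays an ice or fire 2D sound, then sets the target from the State0 (cold) or State2 (hot) marker.
; Tick steps the actor toward the target by Speed per frame, without delta-time scaling or sweep, and snaps on arrival.
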(event EventTick
  (params (DeltaSeconds :type Float%20%28single-precision%29))
  (if (Variables|Default|GetisMoving)
    (if (<= (Math|Vector|Distance(Vector) (Variables|Default|GettargetPos) (Transformation|GetActorLocation (Variables|Default|GetObjectToMove))) (Variables|Default|GetSpeed))
      (Transformation|SetActorLocation (Variables|Default|GetObjectToMove) (Variables|Default|GettargetPos) false false)
      (Variables|Default|SetisMoving false)
      (else
        (Transformation|SetActorLocation (Variables|Default|GetObjectToMove) (+ (* (Math|Vector|Normalize (- (Variables|Default|GettargetPos) (Transformation|GetActorLocation (Variables|Default|GetObjectToMove)))) (Variables|Default|GetSpeed)) (Transformation|GetActorLocation (Variables|Default|GetObjectToMove))) false false)))))

(fn ConstructionScript
  (|CallParentFunction))

(fn SwitchtoColdState
  (Audio|SpawnSound2D "/Game/Music/SoundCues/SFX/SQ_Ice.SQ_Ice" 1.0 1.0 0.0 0)
  (CallFunction|SetNewLocation (Transformation|GetActorLocation (Variables|Default|GetState0Position)))
  (Development|PrintString "Cold"))

(fn SwitchtoHotState
  (Audio|SpawnSound2D "/Game/Music/SoundCues/SFX/SQ_Fire.SQ_Fire" 1.0 1.0 0.0 0)
  (CallFunction|SetNewLocation (Transformation|GetActorLocation (Variables|Default|GetState2Position))))

(fn SetNewLocation
  (params (targetLocation :type Vector))
  (Variables|Default|SettargetPos targetLocation)
  (Variables|Default|SetisMoving true))