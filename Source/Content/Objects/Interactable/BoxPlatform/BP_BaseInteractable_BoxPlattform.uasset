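; Interactable box platform that switches between a solid cold state and a pass-through hot state.
; The cold state gives the cube an ice mesh and material and blocks pawns, while the hot state swaps in the box mesh and material and ignores them.
; Each switch can optionally play its ice or fire sound in 2D.
; An unconnected VFX spawn in the hot-state graph never runs.
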(fn ConstructionScript
  (|CallParentFunction))

(fn SwitchtoColdState
  (params (shouldplaySound :type Boolean))
  (bind _cube (Variables|Default|GetCube))
  (if shouldplaySound
    (Audio|SpawnSound2D "/Game/Music/SoundCues/SFX/SQ_Ice.SQ_Ice" 1.0 1.0 0.0 0))
  (Rendering|Material|SetMaterial _cube 0 "/Game/Levels/PlayGrounds/Kathleen/Material/Mat_IceShader/MAT_TestICE_02_Inst.MAT_TestICE_02_Inst")
  (Collision|SetCollisionResponsetoChannel _cube "ECC_Pawn" "ECR_Block")
  (Components|StaticMesh|SetStaticMesh _cube "/Game/Objects/Plattforms/Meshes/OBJ_BeveledSquareICE_001.OBJ_BeveledSquareICE_001"))

(fn SwitchtoHotState
  (params (shouldplaySound :type Boolean))
  (bind _cube (Variables|Default|GetCube))
  (if shouldplaySound
    (Audio|SpawnSound2D "/Game/Music/SoundCues/SFX/SQ_Fire.SQ_Fire" 1.0 1.0 0.0 0))
  (Rendering|Material|SetMaterial _cube 0 "/Game/Levels/PlayGrounds/Chiara/MAT_Box.MAT_Box")
  (Collision|SetCollisionResponsetoChannel _cube "ECC_Pawn" "ECR_Ignore")
  (Components|StaticMesh|SetStaticMesh _cube "/Game/Objects/Plattforms/Meshes/OBJ_BeveledSquare_002.OBJ_BeveledSquare_002"))