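; Scripted Death actor for a tutorial that, once the player enters its trigger box, travels through waypoints, optionally freezing player movement.
; Tick steps it toward the current Data entry's target, after playing any montage and triggering any interactable with a Niagara lightning beam.
; MadeExtraStuff never resets, so montages and interactions are skipped after the first interaction.
; An entry flagged ShouldDeathDie restores player movement and destroys the actor.
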(event Custom|OnPlayerEntered
  (bind _player (Variables|Default|GetPlayer))
  (Variables|Default|SetIsMoving true)
  (if (Variables|Exposed|GetShouldDisablePlayerMovement)
    (Variables|/Game/Objects/Player/Code/BP_Player.BP_Player_C|SetSpeed _player 0.0)
    (Variables|/Script/Engine.Character|SetJumpMaxCount _player 0)))

(event EventBeginPlay
  (if (Variables|Exposed|GetShouldDeathSpawn)
    (EventDispatchers|BindEventtoPlayerEntered (Variables|Exposed|GetTriggerBox) (EventDispatchers|CreateEvent :!event Custom|OnPlayerEntered))
    (bind _outactors (Actor|GetAllActorsOfClass "/Game/Objects/Player/Code/BP_Player.BP_Player_C"))
    (for _array_element _outactors
      (Variables|Default|SetPlayer _array_element))
    (else
      (Actor|DestroyActor))))

(event EventTick
  (params (DeltaSeconds :type Float%20%28single-precision%29))
  (bind _data (Variables|Exposed|GetData))
  (bind _index (Variables|Default|GetIndex))
  (bind _data_2 (Variables|Exposed|GetData))
  (bind _index_2 (Variables|Default|GetIndex))
  (bind _data_3 (Variables|Exposed|GetData))
  (bind _index_3 (Variables|Default|GetIndex))
  (bind _output (Utilities|Array|Get(acopy) _data _index))
  (bind _output_2 (Utilities|Array|Get(acopy) _data_2 _index_2))
  (bind _output_3 (Utilities|Array|Get(acopy) _data_3 _index_3))
  (if (Variables|Default|GetIsMoving)
    (if (Variables|Default|GetMadeExtraStuff)
      _
      (else
        (if (Utilities|IsValid (.animationtoplay _output_2))
          (Animation|Montage|PlayMontage 0 (.animationtoplay _output_2)
            (:OnCompleted
              _)))
        (Utilities|IsValid (.interactable _output)
          (:Is%20Valid
            (CallFunction|Interact)
            (Variables|Default|SetMadeExtraStuff true)
            (Utilities|FlowControl|Delay 0.5))
          (:Is%20Not%20Valid
            _))))
    (if (<= (Math|Vector|Distance(Vector) (Transformation|GetActorLocation (.targetposition _output)) (Transformation|GetActorLocation)) (.speed _output))
      (Transformation|SetActorLocation (Transformation|GetActorLocation (.targetposition (Utilities|Array|Get(acopy) (Variables|Exposed|GetData) (Variables|Default|GetIndex)))) false false)
      (CallFunction|CheckforNextWaypoint)
      (else
        (Transformation|SetActorLocation (+ (* (Math|Vector|Normalize (- (Transformation|GetActorLocation (.targetposition _output_3)) (Transformation|GetActorLocation))) (.speed _output_3)) (Transformation|GetActorLocation)) false false)))))

(fn ConstructionScript)

(fn CheckforNextWaypoint
  (bind _data (Variables|Exposed|GetData))
  (bind _player (Variables|Default|GetPlayer))
  (if (.shoulddeathdie (Utilities|Array|Get(acopy) (Variables|Exposed|GetData) (Variables|Default|GetIndex)))
    (Variables|Default|SetIsMoving false)
    (Utilities|IsValid _player
      (:Is%20Valid
        (Variables|/Script/Engine.Character|SetJumpMaxCount _player 1)
        (Variables|/Game/Objects/Player/Code/BP_Player.BP_Player_C|SetSpeed _player 1.0))
      (:Is%20Not%20Valid
        _))
    (Actor|DestroyActor)
    (elif (Utilities|Array|ContainsItem _data (Utilities|Array|Get(acopy) _data (+ (Variables|Default|GetIndex) 1)))
      (Variables|Default|SetIndex (+ (Variables|Default|GetIndex) 1)))))

(fn Interact
  (bind _box (Variables|Default|GetBox))
  (bind _index (Variables|Default|GetIndex))
  (bind _data (Variables|Exposed|GetData))
  (bind _returnvalue (Transformation|GetWorldTransform _box))
  (bind _output (Utilities|Array|Get(acopy) _data _index))
  (bind _returnvalue_2 (Transformation|GetActorTransform (.interactable _output)))
  (bind _returnvalue_3 (- (.location _returnvalue_2) (.location _returnvalue)))
  (bind _returnvalue_4 (Math|Vector|Normalize _returnvalue_3))
  (bind _returnvalue_5 (Niagara|SpawnSystematLocation "/Game/Levels/PlayGrounds/Chiara/VFX/Lightning_Em_System1.Lightning_Em_System1" (.location _returnvalue) "0, 0, 0" "1.000000,1.000000,1.000000" true false))
  (Effects|Components|ParticleSystem|SetVectorParameter _returnvalue_5 "User.EndBeam" (* _returnvalue_4 (Math|Vector|Distance(Vector) (.location _returnvalue_2) (.location _returnvalue))))
  (Effects|Components|ParticleSystem|SetVectorParameter _returnvalue_5 "User.PivotPoint" _returnvalue_4)
  (Components|Activation|Activate _returnvalue_5 false)
  (Default|Interact (.interactable (Utilities|Array|Get(acopy) (Variables|Exposed|GetData) (Variables|Default|GetIndex))) "NewEnumerator15"))