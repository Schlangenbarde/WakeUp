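; BP_Projectile is a short-lived projectile that carries a hot or cold heat state to interactable objects.
; Init picks the heat state from an IsCold flag.
; On hit, it passes that state to any BP_BaseInteractable through Interact, then destroys itself regardless of what it struck.
; A FlipFlop on Tick delays showing the sphere until the second frame, then a brief Delay destroys the actor, capping its lifetime.
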(event EventTick
  (params (DeltaSeconds :type Float%20%28single-precision%29))
  (Utilities|FlowControl|FlipFlop
    (:B
      (Rendering|SetVisibility (Variables|Default|GetSphere) true false)
      (Utilities|FlowControl|Delay 0.2)
      (Actor|DestroyActor))))

(event Collision|EventHit
  (params (MyComp :type Primitive%20Component%20Object%20Reference) (Other :type Actor%20Object%20Reference) (OtherComp :type Primitive%20Component%20Object%20Reference) (bSelfMoved :type Boolean) (HitLocation :type Vector :default "0, 0, 0") (HitNormal :type Vector :default "0, 0, 0") (NormalImpulse :type Vector :default "0, 0, 0") (Hit :type Hit%20Result%20Structure%20%28by%20ref%29))
  (bind _asbp_base_interactable (Utilities|Casting|CastToBP_BaseInteractable Other)
    (:then
      (Default|Interact _asbp_base_interactable (Variables|Default|Getheatstate)))
    (:CastFailed
      _))
  (Actor|DestroyActor))

(fn ConstructionScript)

(fn Init
  (params (IsCold :type Boolean))
  (if IsCold
    (Variables|Default|SetheatState "NewEnumerator13")
    (else
      (Variables|Default|SetheatState "NewEnumerator15"))))