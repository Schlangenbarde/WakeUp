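; BP_Bayblade2 is a spinning object that carries four referenced umbrella actors around with it, apparently in the style of a Beyblade top.
; Each Tick sets the RotatingMovement rate from the Rotation variable, then moves each umbrella to the world location of its paired Scene component without sweeping.
; Only location is copied, so the umbrellas do not inherit the spin.
; An alternative snap-attachment chain is present but never runs.
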(event EventBeginPlay)

(event EventTick
  (params (DeltaSeconds :type Float%20%28single-precision%29))
  (Variables|/Script/Engine.RotatingMovementComponent|SetRotationRate (Variables|Default|GetRotatingMovement) (Math|Rotator|MakeRotator 0.0 0.0 (Variables|Default|GetRotation)))
  (Transformation|SetActorLocation (Variables|Default|GetUmbrella) (Transformation|GetWorldLocation (Variables|Default|GetScene1)) false false)
  (Transformation|SetActorLocation (Variables|Default|GetUmbrella_1) (Transformation|GetWorldLocation (Variables|Default|GetScene)) false false)
  (Transformation|SetActorLocation (Variables|Default|GetUmbrella_2) (Transformation|GetWorldLocation (Variables|Default|GetScene3)) false false)
  (Transformation|SetActorLocation (Variables|Default|GetUmbrella_3) (Transformation|GetWorldLocation (Variables|Default|GetScene2)) false false))

(fn ConstructionScript)