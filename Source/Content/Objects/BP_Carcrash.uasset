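; BP_Carcrash is a one-shot scripted car crash triggered by the first overlap with its Box.
; The overlap plays a crash sound, spawns a system at the box and starts movement.
; Tick moves Objects one after another toward matching Position actors by Speed units per frame, without delta-time scaling, then destroys this actor when no valid object remains.
; An unconnected loop with random rotations never runs.
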(event OnComponentBeginOverlap(Box)
  (params (OverlappedComponent :type Primitive%20Component%20Object%20Reference) (OtherActor :type Actor%20Object%20Reference) (OtherComp :type Primitive%20Component%20Object%20Reference) (OtherBodyIndex :type Integer) (bFromSweep :type Boolean) (SweepResult :type Hit%20Result%20Structure%20%28by%20ref%29))
  (Utilities|FlowControl|DoOnce false
    (:Completed
      (Audio|PlaySound2D "/Game/Music/SoundCues/Special/SQ_Carcrash.SQ_Carcrash" 1.0 1.0 0.0 0 0)
      (Niagara|SpawnSystematLocation (Variables|Default|GetSystem%20Template) (Transformation|GetWorldLocation (Variables|Default|GetBox)))
      (Variables|Default|SetisMoving true))))

(event EventTick
  (params (DeltaSeconds :type Float%20%28single-precision%29))
  (bind _objects (Variables|Default|GetObjects))
  (bind _counter (Variables|Default|GetCounter))
  (bind _output (Utilities|Array|Get(acopy) _objects _counter))
  (if (Variables|Default|GetisMoving)
    (if (<= (Math|Vector|Distance(Vector) (Transformation|GetActorLocation (Utilities|Array|Get(acopy) (Variables|Default|GetPosition) (Variables|Default|GetCounter))) (Transformation|GetActorLocation (Utilities|Array|Get(acopy) (Variables|Default|GetObjects) (Variables|Default|GetCounter)))) (Variables|Default|GetSpeed))
      (Transformation|SetActorLocation (Utilities|Array|Get(acopy) (Variables|Default|GetObjects) (Variables|Default|GetCounter)) (Transformation|GetActorLocation (Utilities|Array|Get(acopy) (Variables|Default|GetPosition) (Variables|Default|GetCounter))) false false)
      (bind _result (Math|Integer|IncrementInt (Variables|Default|GetCounter))
        (:%20%20
          (Utilities|IsValid (Utilities|Array|Get(acopy) (Variables|Default|GetObjects) _result)
            (:Is%20Not%20Valid
              (Variables|Default|SetisMoving false)
              (Actor|DestroyActor)))))
      (else
        (Transformation|SetActorLocation _output (+ (* (Math|Vector|Normalize (- (Transformation|GetActorLocation (Utilities|Array|Get(acopy) (Variables|Default|GetPosition) (Variables|Default|GetCounter))) (Transformation|GetActorLocation _output))) (Variables|Default|GetSpeed)) (Transformation|GetActorLocation _output)) false false)))))

(fn ConstructionScript)