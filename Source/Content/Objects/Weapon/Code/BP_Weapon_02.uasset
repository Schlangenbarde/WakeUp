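; BP_Weapon_02 is a pickup weapon that, on player overlap, attaches to the hot weapon slot, binds both fire events and removes its trigger and rotation.
; Cold and hot shots share a brief cooldown and line trace from the player camera, sending a type-specific interaction to any BP_BaseInteractable hit.
; Each shot spawns an ice or lightning beam at the muzzle child actor, aimed through vector parameters.
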(event OnComponentBeginOverlap(Box)
  (params (OverlappedComponent :type Primitive%20Component%20Object%20Reference) (OtherActor :type Actor%20Object%20Reference) (OtherComp :type Primitive%20Component%20Object%20Reference) (OtherBodyIndex :type Integer) (bFromSweep :type Boolean) (SweepResult :type Hit%20Result%20Structure%20%28by%20ref%29))
  (bind _asbp_player (Utilities|Casting|CastToBP_Player OtherActor))
  (bind _output_get (Variables|Default|Setplayer _asbp_player))
  (EventDispatchers|BindEventtoUseColdWeapon _output_get (EventDispatchers|CreateEvent :!event Custom|ShootCold))
  (EventDispatchers|BindEventtoUseHotWeapon _output_get (EventDispatchers|CreateEvent :!event Custom|ShootHot))
  (Transformation|AttachComponentToComponent (Variables|/Game/Objects/Player/Code/BP_Player.BP_Player_C|GetHotWeaponSlot _output_get) "None" "SnapToTarget" "SnapToTarget" "SnapToTarget" true)
  (Components|DestroyComponent (Variables|Default|GetRotatingMovement))
  (Components|DestroyComponent (Variables|Default|GetBox))
  (Utilities|Array|Add (Variables|Default|GetActors%20to%20Ignore) (Variables|Default|Getplayer)))

(event Custom|ShootCold
  (if (not (Variables|Default|GetisCoolDownActive))
    (bind _hitactor (CallFunction|Shoot true))
    (bind _asbp_base_interactable (Utilities|Casting|CastToBP_BaseInteractable _hitactor)
      (:then
        (Default|Interact _asbp_base_interactable "NewEnumerator13"))
      (:CastFailed
        _))
    (Variables|Default|SetisCoolDownActive true)
    (Utilities|FlowControl|Delay 0.63)
    (Variables|Default|SetisCoolDownActive false)))

(event Custom|ShootHot
  (if (not (Variables|Default|GetisCoolDownActive))
    (bind _hitactor (CallFunction|Shoot false))
    (bind _asbp_base_interactable (Utilities|Casting|CastToBP_BaseInteractable _hitactor)
      (:then
        (Default|Interact _asbp_base_interactable "NewEnumerator15"))
      (:CastFailed
        _))
    (Variables|Default|SetisCoolDownActive true)
    (Utilities|FlowControl|Delay 0.63)
    (Variables|Default|SetisCoolDownActive false)))

(fn ConstructionScript)

(fn Shoot
  (params (IsColdShot :type Boolean))
  (bind _distance (Variables|Default|GetDistance))
  (bind _player (Variables|Default|Getplayer))
  (bind _returnvalue (Math|Conversions|ToVector(Float) _distance))
  (bind _camera (Variables|/Game/Objects/Player/Code/BP_Player.BP_Player_C|GetCamera _player))
  (bind _returnvalue_2 (Transformation|GetWorldLocation _camera))
  (bind _returnvalue_3 (Transformation|GetWorldRotation _camera))
  (bind _returnvalue_4 (Math|Vector|GetForwardVector _returnvalue_3))
  (bind _returnvalue_5 (* _returnvalue_4 _returnvalue))
  (bind _returnvalue_6 (+ _returnvalue_2 _returnvalue_5))
  (bind _outhit (Collision|LineTraceByChannel _returnvalue_2 _returnvalue_6 "TraceTypeQuery2" false (Variables|Default|GetActors%20to%20Ignore) "ForDuration"))
  (if IsColdShot
    (CallFunction|PlayEffect _returnvalue_6 "/Game/Levels/PlayGrounds/Chiara/VFX/IceBeam_Emiter_System1.IceBeam_Emiter_System1")
    (else
      (CallFunction|PlayEffect _returnvalue_6 "/Game/Levels/PlayGrounds/Chiara/VFX/Lightning_Em_System1.Lightning_Em_System1")))
  (return (.HitActor (Collision|BreakHitResult _outhit))))

(fn PlayEffect
  (params (End :type Vector) (SystemTemplate :type Niagara%20System%20Object%20Reference))
  (bind _childactor1 (Variables|Default|GetChildActor1))
  (bind _returnvalue (Transformation|GetWorldTransform _childactor1))
  (bind _returnvalue_2 (- End (.location _returnvalue)))
  (bind _returnvalue_3 (Math|Vector|Normalize _returnvalue_2))
  (bind _returnvalue_4 (Niagara|SpawnSystematLocation SystemTemplate (.location _returnvalue) "0, 0, 0" "1.000000,1.000000,1.000000" true false))
  (Effects|Components|ParticleSystem|SetVectorParameter _returnvalue_4 "User.EndBeam" (* _returnvalue_3 (Variables|Default|GetDistance)))
  (Effects|Components|ParticleSystem|SetVectorParameter _returnvalue_4 "User.PivotPoint" _returnvalue_3)
  (Effects|Components|ParticleSystem|SetVectorParameter _returnvalue_4 "User.BoxSize" (Math|Vector|MakeVector 0.0 1e+01 1e+01))
  (Components|Activation|Activate _returnvalue_4 false))