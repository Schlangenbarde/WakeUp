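; Main weapon pickup that gives the player hot and cold beam shots for changing the heat state of interactables.
; On overlap it plays an optional montage, updates an existing save slot, binds to player fire events and attaches to the hot weapon slot.
; Shots share a cooldown and line trace toward the camera aim, cold from the drone, calling Interact on hit interactables.
; Beam effects are stretched to the target through User parameters.
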(event OnComponentBeginOverlap(Box)
  (params (OverlappedComponent :type Primitive%20Component%20Object%20Reference) (OtherActor :type Actor%20Object%20Reference) (OtherComp :type Primitive%20Component%20Object%20Reference) (OtherBodyIndex :type Integer) (bFromSweep :type Boolean) (SweepResult :type Hit%20Result%20Structure%20%28by%20ref%29))
  (bind _animationtoplay (Variables|Default|GetAnimationToPlay))
  (bind _asbp_player (Utilities|Casting|CastToBP_Player OtherActor))
  (Utilities|IsValid _animationtoplay
    (:Is%20Valid
      (Animation|Montage|PlayMontage 0 _animationtoplay
        (:OnCompleted
          _)))
    (:Is%20Not%20Valid
      _))
  (CallFunction|SaveGame)
  (CallFunction|BindtoPlayer _asbp_player))

(event Custom|ShootHot
  (bind _player (Variables|Default|Getplayer))
  (bind _camera (Variables|/Game/Objects/Player/Code/BP_Player.BP_Player_C|GetCamera _player))
  (bind _returnvalue (Transformation|GetWorldLocation _camera))
  (if (not (Variables|Default|GetIs%20Cool%20Down%20Active))
    (Audio|PlaySound2D "/Game/Music/SoundCues/SFX/SC_ShootHot.SC_ShootHot" 1.0 1.0 0.0 0 0)
    (bind _hitactor (CallFunction|Shoot "/Game/Levels/PlayGrounds/Chiara/VFX/Lightning_Em_System1.Lightning_Em_System1" "/Game/Levels/PlayGrounds/Chiara/VFX/Lightning_Hit.Lightning_Hit" _returnvalue (+ _returnvalue (* (Math|Vector|GetForwardVector (Transformation|GetWorldRotation _camera)) (Math|Conversions|ToVector(Float) (Variables|Default|GetDistance)))) (Variables|Default|Gettriangle_Triangle) "NewEnumerator15" "/Game/Levels/PlayGrounds/Chiara/VFX/Lightning+Ice_Hit.Lightning+Ice_Hit"))
    (bind _asbp_base_interactable (Utilities|Casting|CastToBP_BaseInteractable _hitactor)
      (:then
        (Default|Interact _asbp_base_interactable "NewEnumerator15"))
      (:CastFailed
        _))
    (Variables|Default|SetIs%20Cool%20Down%20Active true)
    (Utilities|FlowControl|Delay 0.63)
    (Variables|Default|SetIs%20Cool%20Down%20Active false)))

(event Custom|ShootCold
  (bind _player (Variables|Default|Getplayer))
  (bind _drone_rework (Variables|Default|GetDrone_Rework))
  (bind _camera (Variables|/Game/Objects/Player/Code/BP_Player.BP_Player_C|GetCamera _player))
  (if (not (Variables|Default|GetIs%20Cool%20Down%20Active))
    (Audio|PlaySound2D "/Game/Music/SoundCues/SFX/SC_ShootCold.SC_ShootCold" 1.0 1.0 0.0 0 0)
    (bind _hitactor (CallFunction|Shoot "/Game/Levels/PlayGrounds/Chiara/VFX/IceBeam_Emiter_System1.IceBeam_Emiter_System1" "/Game/Levels/PlayGrounds/Chiara/VFX/IceBeam_Hit.IceBeam_Hit" (Transformation|GetWorldLocation _drone_rework) (+ (Transformation|GetWorldLocation _camera) (* (Math|Vector|GetForwardVector (Transformation|GetWorldRotation _camera)) (Math|Conversions|ToVector(Float) (Variables|Default|GetDistance)))) _drone_rework "NewEnumerator13" "/Game/Levels/PlayGrounds/Chiara/VFX/IceBeam_Hit.IceBeam_Hit"))
    (bind _asbp_base_interactable (Utilities|Casting|CastToBP_BaseInteractable _hitactor)
      (:then
        (Default|Interact _asbp_base_interactable "NewEnumerator13"))
      (:CastFailed
        _))
    (Variables|Default|SetIs%20Cool%20Down%20Active true)
    (Utilities|FlowControl|Delay 0.63)
    (Variables|Default|SetIs%20Cool%20Down%20Active false)))

(event EventBindtoPlayer
  (params (Player :type BP%20Player%20Object%20Reference))
  (bind _box (Variables|Default|GetBox))
  (bind _output_get (Variables|Default|Setplayer Player))
  (Variables|/Game/Objects/Player/Code/BP_Player.BP_Player_C|SetWeapon _output_get self)
  (EventDispatchers|BindEventtoUseHotWeapon _output_get (EventDispatchers|CreateEvent :!event Custom|ShootHot))
  (EventDispatchers|BindEventtoUseColdWeapon _output_get (EventDispatchers|CreateEvent :!event Custom|ShootCold))
  (Transformation|AttachComponentToComponent (Variables|/Game/Objects/Player/Code/BP_Player.BP_Player_C|GetHotWeaponSlot _output_get) "None" "SnapToTarget" "SnapToTarget" "SnapToTarget" true)
  (Utilities|IsValid _box
    (:Is%20Valid
      (Components|DestroyComponent _box))
    (:Is%20Not%20Valid
      _))
  (Utilities|Array|Add (Variables|Default|GetActors%20to%20Ignore) (Variables|Default|Getplayer)))

(fn ConstructionScript)

(fn Shoot
  (params (Beam%20Effect :type Niagara%20System%20Object%20Reference) (Hit%20Effect :type Niagara%20System%20Object%20Reference) (Start :type Vector) (End :type Vector) (start%20actor :type Scene%20Component%20Object%20Reference) (HeatState :type ENUM_HeatState%20Enum :default "NewEnumerator13") (SpecialEffect :type Niagara%20System%20Object%20Reference))
  (bind (_outhit _returnvalue) (Collision|LineTraceByChannel Start End "TraceTypeQuery2" false (Variables|Default|GetActors%20to%20Ignore) "None"))
  (if _returnvalue
    (bind _asbp_base_interactable (Utilities|Casting|CastToBP_BaseInteractable (.HitActor (Collision|BreakHitResult _outhit)))
      (:then
        (if (== (Variables|/Game/Objects/Interactable/Code/BP_BaseInteractable.BP_BaseInteractable_C|GetHeat%20State _asbp_base_interactable) HeatState)
          _
          (else
            (Niagara|SpawnSystematLocation SpecialEffect (.ImpactPoint (Collision|BreakHitResult _outhit))))))
      (:CastFailed
        _))
    (CallFunction|PlayEffect (.ImpactPoint (Collision|BreakHitResult _outhit)) Beam%20Effect start%20actor)
    (bind _returnvalue_2 (Niagara|SpawnSystematLocation Hit%20Effect (.ImpactPoint (Collision|BreakHitResult _outhit)) "0, 0, 0" "1.000000,1.000000,1.000000" true false))
    (Components|Activation|Activate _returnvalue_2 false)
    (else
      (CallFunction|PlayEffect End Beam%20Effect start%20actor)))
  (return (.HitActor (Collision|BreakHitResult _outhit))))

(fn SaveGame
  (bind _returnvalue (SaveGame|DoesSaveGameExist "MyCoolSlot"))
  (if _returnvalue
    (bind _returnvalue_2 (SaveGame|LoadGamefromSlot "MyCoolSlot"))
    (bind _asbp_save_game_save_slot_one (Utilities|Casting|CastToBP_SaveGame_SaveSlotOne _returnvalue_2))
    (Variables|/Game/Data/SaveClasses/BP_SaveGame_SaveSlotOne.BP_SaveGame_SaveSlotOne_C|SetData _asbp_save_game_save_slot_one (Utilities|Struct|MakeSTRUCT_SaveSlotOneData (.checkpointposition (Variables|/Game/Data/SaveClasses/BP_SaveGame_SaveSlotOne.BP_SaveGame_SaveSlotOne_C|GetData _asbp_save_game_save_slot_one)) (.lastlevel (Variables|/Game/Data/SaveClasses/BP_SaveGame_SaveSlotOne.BP_SaveGame_SaveSlotOne_C|GetData _asbp_save_game_save_slot_one)) (.shouldloadlastcheckpoint (Variables|/Game/Data/SaveClasses/BP_SaveGame_SaveSlotOne.BP_SaveGame_SaveSlotOne_C|GetData _asbp_save_game_save_slot_one)) true "NewEnumerator2"))
    (SaveGame|SaveGametoSlot _returnvalue_2 "MyCoolSlot")))

(fn PlayEffect
  (params (End :type Vector) (SystemTemplate :type Niagara%20System%20Object%20Reference) (start%20actor :type Scene%20Component%20Object%20Reference))
  (bind _returnvalue (Transformation|GetWorldTransform start%20actor))
  (bind _returnvalue_2 (Math|Rotator|FindLookatRotation (.location _returnvalue) End))
  (bind _returnvalue_3 (Niagara|SpawnSystematLocation SystemTemplate (.location _returnvalue) "0, 0, 0" "1.000000,1.000000,1.000000" true false))
  (Effects|Components|ParticleSystem|SetVectorParameter _returnvalue_3 "User.EndBeam" (* (Math|Vector|Normalize (- End (.location _returnvalue))) (Math|Vector|Distance(Vector) End (.location _returnvalue))))
  (Effects|Components|ParticleSystem|SetVectorParameter _returnvalue_3 "User.Rotation" (Math|Vector|MakeVector (.yaw _returnvalue_2) (.pitch _returnvalue_2) (.roll _returnvalue_2)))
  (Effects|Components|ParticleSystem|SetVectorParameter _returnvalue_3 "User.BoxSize" (Math|Vector|MakeVector (Variables|Default|GetDistance) 1e+01 1e+01))
  (Components|Activation|Activate _returnvalue_3 false))