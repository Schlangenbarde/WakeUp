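; BP_ColdWeapon is a weapon pickup that triggers when the player overlaps its box.
; It plays an optional montage, then on completion plays a sound, saves and binds to the player.
; Saving updates an existing save slot's flag and enum fields, keeping checkpoint and level data.
; Binding has the player check its weapon, binds MainWeapon to the player and destroys the pickup actor.
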(event OnComponentBeginOverlap(Box)
  (params (OverlappedComponent :type Primitive%20Component%20Object%20Reference) (OtherActor :type Actor%20Object%20Reference) (OtherComp :type Primitive%20Component%20Object%20Reference) (OtherBodyIndex :type Integer) (bFromSweep :type Boolean) (SweepResult :type Hit%20Result%20Structure%20%28by%20ref%29))
  (bind _animation_to_play (Variables|Default|GetAnimation%20to%20Play))
  (bind _asbp_player (Utilities|Casting|CastToBP_Player OtherActor))
  (Utilities|IsValid _animation_to_play
    (:Is%20Valid
      (Animation|Montage|PlayMontage 0 _animation_to_play
        (:OnCompleted
          _)))
    (:Is%20Not%20Valid
      _))
  (Audio|PlaySound2D (Variables|Default|GetSound) 1.0 1.0 0.0 0 0)
  (CallFunction|Save)
  (CallFunction|BindtoPlayer _asbp_player))

(fn ConstructionScript)

(fn BindtoPlayer
  (params (player :type BP%20Player%20Object%20Reference))
  (bind _output_get (Variables|Default|SetPlayer player))
  (Default|CheckWeapon _output_get)
  (Default|BindtoPlayer (Variables|Default|GetMainWeapon) _output_get)
  (Actor|DestroyActor))

(fn Save
  (bind _returnvalue (SaveGame|DoesSaveGameExist "MyCoolSlot"))
  (if _returnvalue
    (bind _returnvalue_2 (SaveGame|LoadGamefromSlot "MyCoolSlot"))
    (bind _asbp_save_game_save_slot_one (Utilities|Casting|CastToBP_SaveGame_SaveSlotOne _returnvalue_2))
    (Variables|/Game/Data/SaveClasses/BP_SaveGame_SaveSlotOne.BP_SaveGame_SaveSlotOne_C|SetData _asbp_save_game_save_slot_one (Utilities|Struct|MakeSTRUCT_SaveSlotOneData (.checkpointposition (Variables|/Game/Data/SaveClasses/BP_SaveGame_SaveSlotOne.BP_SaveGame_SaveSlotOne_C|GetData _asbp_save_game_save_slot_one)) (.lastlevel (Variables|/Game/Data/SaveClasses/BP_SaveGame_SaveSlotOne.BP_SaveGame_SaveSlotOne_C|GetData _asbp_save_game_save_slot_one)) (.shouldloadlastcheckpoint (Variables|/Game/Data/SaveClasses/BP_SaveGame_SaveSlotOne.BP_SaveGame_SaveSlotOne_C|GetData _asbp_save_game_save_slot_one)) true "NewEnumerator2"))
    (SaveGame|SaveGametoSlot _returnvalue_2 "MyCoolSlot")))