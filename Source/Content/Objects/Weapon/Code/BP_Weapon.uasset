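; Pickup for the player's hot weapon, which fires a lightning beam that triggers interactable objects.
; On player overlap it plays an optional montage, attaches to the hot weapon slot, records the pickup in an existing save and refreshes the UI.
; Firing, bound to a player event, line-traces from the camera under a short cooldown and calls Interact on hit BP_BaseInteractable actors.
; Niagara parameters stretch the beam from the muzzle child actor to the trace end.
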(event OnComponentBeginOverlap(Box)
  (params (OverlappedComponent :type Primitive%20Component%20Object%20Reference) (OtherActor :type Actor%20Object%20Reference) (OtherComp :type Primitive%20Component%20Object%20Reference) (OtherBodyIndex :type Integer) (bFromSweep :type Boolean) (SweepResult :type Hit%20Result%20Structure%20%28by%20ref%29))
  (bind _animationtoplay (Variables|Default|GetAnimationToPlay))
  (bind _asbp_player (Utilities|Casting|CastToBP_Player OtherActor))
  (Utilities|IsValid _animationtoplay
    (:Is%20Valid
      (Animation|Montage|PlayMontage 0 _animationtoplay
        (:OnCompleted
          _)))
    (:Is%20Not%20Valid
      _))
  (Audio|PlaySound2D (Variables|Default|GetSound) 1.0 1.0 0.0 0 0)
  (CallFunction|BindtoPlayer _asbp_player)
  (CallFunction|SaveGame)
  (Default|Setup (Variables|/Game/Objects/Player/Code/BP_Player.BP_Player_C|GetPlayerUI _asbp_player)))

(event Custom|ShootHot
  (if (not (Variables|Default|GetisCoolDownActive))
    (bind _hitactor (CallFunction|Shoot))
    (bind _asbp_base_interactable (Utilities|Casting|CastToBP_BaseInteractable _hitactor)
      (:then
        (Default|Interact _asbp_base_interactable "NewEnumerator15"))
      (:CastFailed
        _))
    (Variables|Default|SetisCoolDownActive true)
    (Utilities|FlowControl|Delay 0.63)
    (Variables|Default|SetisCoolDownActive false)))

(event EventBindtoPlayer
  (params (Player :type BP%20Player%20Object%20Reference))
  (bind _output_get (Variables|Default|Setplayer Player))
  (Variables|/Game/Objects/Player/Code/BP_Player.BP_Player_C|SetWeapon _output_get self)
  (EventDispatchers|BindEventtoUseHotWeapon _output_get (EventDispatchers|CreateEvent :!event Custom|ShootHot))
  (Transformation|AttachComponentToComponent (Variables|/Game/Objects/Player/Code/BP_Player.BP_Player_C|GetHotWeaponSlot _output_get) "None" "SnapToTarget" "SnapToTarget" "SnapToTarget" true)
  (Components|DestroyComponent (Variables|Default|GetRotatingMovement))
  (Components|DestroyComponent (Variables|Default|GetBox))
  (Utilities|Array|Add (Variables|Default|GetActors%20to%20Ignore) (Variables|Default|Getplayer)))

(fn ConstructionScript)

(fn Shoot
  (bind _distance (Variables|Default|GetDistance))
  (bind _player (Variables|Default|Getplayer))
  (bind _returnvalue (Math|Conversions|ToVector(Float) _distance))
  (bind _camera (Variables|/Game/Objects/Player/Code/BP_Player.BP_Player_C|GetCamera _player))
  (bind _returnvalue_2 (Transformation|GetWorldLocation _camera))
  (bind _returnvalue_3 (Transformation|GetWorldRotation _camera))
  (bind _returnvalue_4 (Math|Vector|GetForwardVector _returnvalue_3))
  (bind _returnvalue_5 (* _returnvalue_4 _returnvalue))
  (bind _returnvalue_6 (+ _returnvalue_2 _returnvalue_5))
  (bind (_outhit _returnvalue_7) (Collision|LineTraceByChannel _returnvalue_2 _returnvalue_6 "TraceTypeQuery2" false (Variables|Default|GetActors%20to%20Ignore) "None"))
  (if _returnvalue_7
    (CallFunction|PlayEffect (.ImpactPoint (Collision|BreakHitResult _outhit)) "/Game/Levels/PlayGrounds/Chiara/VFX/Lightning_Em_System1.Lightning_Em_System1")
    (bind _returnvalue_8 (Niagara|SpawnSystematLocation "/Game/Levels/PlayGrounds/Chiara/VFX/Lightning_Hit.Lightning_Hit" (.ImpactPoint (Collision|BreakHitResult _outhit)) "0, 0, 0" "1.000000,1.000000,1.000000" true false))
    (Components|Activation|Activate _returnvalue_8 false)
    (else
      (CallFunction|PlayEffect _returnvalue_6 "/Game/Levels/PlayGrounds/Chiara/VFX/Lightning_Em_System1.Lightning_Em_System1")))
  (return (.HitActor (Collision|BreakHitResult _outhit))))

(fn PlayEffect
  (params (End :type Vector) (SystemTemplate :type Niagara%20System%20Object%20Reference))
  (bind _childactor1 (Variables|Default|GetChildActor1))
  (bind _returnvalue (Transformation|GetWorldTransform _childactor1))
  (bind _returnvalue_2 (Math|Rotator|FindLookatRotation (.location _returnvalue) End))
  (bind _returnvalue_3 (Niagara|SpawnSystematLocation SystemTemplate (.location _returnvalue) "0, 0, 0" "1.000000,1.000000,1.000000" true false))
  (Effects|Components|ParticleSystem|SetVectorParameter _returnvalue_3 "User.EndBeam" (* (Math|Vector|Normalize (- End (.location _returnvalue))) (Math|Vector|Distance(Vector) End (.location _returnvalue))))
  (Effects|Components|ParticleSystem|SetVectorParameter _returnvalue_3 "User.Rotation" (Math|Vector|MakeVector (.yaw _returnvalue_2) (.pitch _returnvalue_2) (.roll _returnvalue_2)))
  (Effects|Components|ParticleSystem|SetVectorParameter _returnvalue_3 "User.BoxSize" (Math|Vector|MakeVector (Variables|Default|GetDistance) 1e+01 1e+01))
  (Components|Activation|Activate _returnvalue_3 false)
  (Audio|PlaySound2D "/Game/Music/SoundCues/SFX/SC_ShootHot.SC_ShootHot" 1.0 1.0 0.0 0 0))

(fn SaveGame
  (bind _returnvalue (SaveGame|DoesSaveGameExist "MyCoolSlot"))
  (if _returnvalue
    (bind _returnvalue_2 (SaveGame|LoadGamefromSlot "MyCoolSlot"))
    (bind _asbp_save_game_save_slot_one (Utilities|Casting|CastToBP_SaveGame_SaveSlotOne _returnvalue_2))
    (Variables|/Game/Data/SaveClasses/BP_SaveGame_SaveSlotOne.BP_SaveGame_SaveSlotOne_C|SetData _asbp_save_game_save_slot_one (Utilities|Struct|MakeSTRUCT_SaveSlotOneData (.checkpointposition (Variables|/Game/Data/SaveClasses/BP_SaveGame_SaveSlotOne.BP_SaveGame_SaveSlotOne_C|GetData _asbp_save_game_save_slot_one)) (.lastlevel (Variables|/Game/Data/SaveClasses/BP_SaveGame_SaveSlotOne.BP_SaveGame_SaveSlotOne_C|GetData _asbp_save_game_save_slot_one)) (.shouldloadlastcheckpoint (Variables|/Game/Data/SaveClasses/BP_SaveGame_SaveSlotOne.BP_SaveGame_SaveSlotOne_C|GetData _asbp_save_game_save_slot_one)) true "NewEnumerator1"))
    (SaveGame|SaveGametoSlot _returnvalue_2 "MyCoolSlot")))