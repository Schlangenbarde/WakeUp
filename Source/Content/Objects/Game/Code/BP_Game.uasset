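; BP_Game is a game manager actor that handles checkpoints, player resets and save progress.
; On BeginPlay it finds the player, binds to every checkpoint and reset box, then restores the saved weapon and, if flagged, checkpoint position.
; Checkpoint activation writes position and level name to a single save slot, clearing the load flag.
; Reset boxes teleport the player above the last checkpoint; saved positions apply only in the matching level.
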(event Custom|ActivateCheckpoint
  (params (NewParam :type BP%20Checkpoint%20Object%20Reference))
  (Variables|Default|SetlastCheckpoint NewParam)
  (Development|PrintString "Checkpoint triggerd")
  (bind _returnvalue (SaveGame|DoesSaveGameExist "MyCoolSlot"))
  (bind _returnvalue_2 (Game|GetCurrentLevelName true))
  (if _returnvalue
    (CallFunction|OverrideSaveData (Transformation|GetWorldLocation (Variables|/Game/Objects/Checkpoint/Code/BP_Checkpoint.BP_Checkpoint_C|GetBox (Variables|Default|GetlastCheckpoint))) _returnvalue_2)
    (else
      (CallFunction|CreateSaveData (Transformation|GetWorldLocation (Variables|/Game/Objects/Checkpoint/Code/BP_Checkpoint.BP_Checkpoint_C|GetBox (Variables|Default|GetlastCheckpoint))) _returnvalue_2))))

(event Custom|ResetPlayer
  (params (Target :type Actor%20Object%20Reference))
  (bind _lastcheckpoint (Variables|Default|GetlastCheckpoint))
  (if (Utilities|IsValid _lastcheckpoint)
    (bind _returnvalue (Game|GetCurrentLevelName true))
    (CallFunction|ResetActortoLastCheckPoint (+ (Transformation|GetWorldLocation (Variables|/Game/Objects/Checkpoint/Code/BP_Checkpoint.BP_Checkpoint_C|GetBox _lastcheckpoint)) (Math|Vector|MakeVector 0.0 0.0 (Variables|Default|GetFallingHigfht))) _returnvalue)))

(event EventBeginPlay
  (Utilities|FlowControl|Sequence
    (:then_0
      (bind _asbp_player (Utilities|Casting|CastToBP_PlayerClass "/Game/Objects/Player/Code/BP_Player.BP_Player_C"))
      (bind _outactors (Actor|GetAllActorsOfClass _asbp_player))
      (for _array_element _outactors
        (Variables|Default|SetPlayer _array_element)))
    (:then_1
      (bind _asbp_checkpoint (Utilities|Casting|CastToBP_CheckpointClass "/Game/Objects/Checkpoint/Code/BP_Checkpoint.BP_Checkpoint_C"))
      (bind _outactors_2 (Actor|GetAllActorsOfClass _asbp_checkpoint))
      (for _array_element_2 _outactors_2
        (EventDispatchers|BindEventtoOnPlayerEnabled _array_element_2 (EventDispatchers|CreateEvent :!event Custom|ActivateCheckpoint)))
      (bind _asbp_reset_box (Utilities|Casting|CastToBP_ResetBoxClass "/Game/Objects/ResetBox/Code/BP_ResetBox.BP_ResetBox_C"))
      (bind _outactors_3 (Actor|GetAllActorsOfClass _asbp_reset_box))
      (for _array_element_3 _outactors_3
        (EventDispatchers|BindEventtoOnPlayerReset _array_element_3 (EventDispatchers|CreateEvent :!event Custom|ResetPlayer)))
      (bind _returnvalue (SaveGame|DoesSaveGameExist "MyCoolSlot"))
      (if _returnvalue
        (bind _returnvalue_2 (SaveGame|LoadGamefromSlot "MyCoolSlot"))
        (bind _asbp_save_game_save_slot_one (Utilities|Casting|CastToBP_SaveGame_SaveSlotOne _returnvalue_2))
        (if (.shouldloadlastcheckpoint (Variables|/Game/Data/SaveClasses/BP_SaveGame_SaveSlotOne.BP_SaveGame_SaveSlotOne_C|GetData _asbp_save_game_save_slot_one))
          (CallFunction|ResetActortoLastCheckPoint (.checkpointposition (Variables|/Game/Data/SaveClasses/BP_SaveGame_SaveSlotOne.BP_SaveGame_SaveSlotOne_C|GetData _asbp_save_game_save_slot_one)) (.lastlevel (Variables|/Game/Data/SaveClasses/BP_SaveGame_SaveSlotOne.BP_SaveGame_SaveSlotOne_C|GetData _asbp_save_game_save_slot_one))))
        (if (.playercollectedweapon (Variables|/Game/Data/SaveClasses/BP_SaveGame_SaveSlotOne.BP_SaveGame_SaveSlotOne_C|GetData _asbp_save_game_save_slot_one))
          (switch Utilities|FlowControl|Switch|SwitchonENUM_WeaponState (.weapon (Variables|/Game/Data/SaveClasses/BP_SaveGame_SaveSlotOne.BP_SaveGame_SaveSlotOne_C|GetData _asbp_save_game_save_slot_one))
            (:NewEnumerator1
              (Default|BindtoPlayer (Variables|Default|GetWeapon) (Variables|Default|GetPlayer)))
            (:NewEnumerator2
              (Default|BindtoPlayer (Variables|Default|GetMainWeapon) (Variables|Default|GetPlayer)))))))))

(fn ConstructionScript)

(fn ResetActortoLastCheckPoint
  (params (NewLocation :type Vector) (lvlNamen :type String))
  (bind _returnvalue (Game|GetCurrentLevelName true))
  (if (== (Utilities|String|StringToName _returnvalue) (Utilities|String|StringToName lvlNamen))
    (Transformation|SetActorLocation (Variables|Default|GetPlayer) NewLocation false false)))

(fn OverrideSaveData
  (params (Checkpoint :type Vector) (Data%20Last%20Level :type String))
  (bind _returnvalue (SaveGame|LoadGamefromSlot "MyCoolSlot"))
  (bind _asbp_save_game_save_slot_one (Utilities|Casting|CastToBP_SaveGame_SaveSlotOne _returnvalue))
  (Variables|/Game/Data/SaveClasses/BP_SaveGame_SaveSlotOne.BP_SaveGame_SaveSlotOne_C|SetData _asbp_save_game_save_slot_one (Utilities|Struct|MakeSTRUCT_SaveSlotOneData Checkpoint Data%20Last%20Level false (.playercollectedweapon (Variables|/Game/Data/SaveClasses/BP_SaveGame_SaveSlotOne.BP_SaveGame_SaveSlotOne_C|GetData _asbp_save_game_save_slot_one)) (.weapon (Variables|/Game/Data/SaveClasses/BP_SaveGame_SaveSlotOne.BP_SaveGame_SaveSlotOne_C|GetData _asbp_save_game_save_slot_one))))
  (SaveGame|SaveGametoSlot _returnvalue "MyCoolSlot"))

(fn CreateSaveData
  (params (Data%20Check%20Point%20Position :type Vector) (Data%20Last%20Level :type String))
  (bind _returnvalue (SaveGame|CreateSaveGameObject "/Game/Data/SaveClasses/BP_SaveGame_SaveSlotOne.BP_SaveGame_SaveSlotOne_C"))
  (Variables|/Game/Data/SaveClasses/BP_SaveGame_SaveSlotOne.BP_SaveGame_SaveSlotOne_C|SetData _returnvalue (Utilities|Struct|MakeSTRUCT_SaveSlotOneData Data%20Check%20Point%20Position Data%20Last%20Level false false "NewEnumerator0"))
  (SaveGame|SaveGametoSlot _returnvalue "MyCoolSlot"))