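; BP_BaseCollectable_Win is the win trigger that returns the player to the main menu once all collectables are gathered.
; On BeginPlay it binds to CollectionOfCollectables' OnAllCollected event, which sets the IsAllCollected flag.
; When BP_Player overlaps its Box and that flag is set, it opens LVL_MainMenu.
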(event OnComponentBeginOverlap(Box)
  (params (OverlappedComponent :type Primitive%20Component%20Object%20Reference) (OtherActor :type Actor%20Object%20Reference) (OtherComp :type Primitive%20Component%20Object%20Reference) (OtherBodyIndex :type Integer) (bFromSweep :type Boolean) (SweepResult :type Hit%20Result%20Structure%20%28by%20ref%29))
  (Utilities|Casting|CastToBP_Player OtherActor)
  (if (Variables|Default|GetisAllCollected)
    (Game|OpenLevel(byObjectReference) "/Game/Levels/Menu/Main/LVL_MainMenu.LVL_MainMenu")))

(event Custom|OnAllCollected
  (Variables|Default|SetisAllCollected true))

(event EventBeginPlay
  (EventDispatchers|BindEventtoOnAllCollected (Variables|Default|GetCollectionOfCollectables) (EventDispatchers|CreateEvent :!event Custom|OnAllCollected)))

(fn ConstructionScript
  (|CallParentFunction))