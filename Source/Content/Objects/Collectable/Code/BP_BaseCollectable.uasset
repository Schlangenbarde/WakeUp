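; BP_BaseCollectable is the base Blueprint for collectable objects, handling what happens when one is interacted with.
; Interact calls the OnCollected dispatcher, then plays two 2D sounds, CollectSound and Sound.
; It casts its root component's owner back to BP_BaseCollectable to broadcast OnCollectedBySelf with that reference.
; Interact returns the duration of Sound, and nothing here hides or destroys the actor.
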(fn ConstructionScript)

(fn Interact
  (bind _sound (Variables|Default|GetSound))
  (Default|CallOnCollected)
  (Audio|PlaySound2D (Variables|Default|GetCollectSound) 1.0 1.0 0.0 0 0)
  (Audio|PlaySound2D _sound 1.0 1.0 0.0 0 0)
  (bind _asbp_base_collectable (Utilities|Casting|CastToBP_BaseCollectable (Components|GetOwner (Variables|Default|GetDefaultSceneRoot)))
    (:then
      (Default|CallOnCollectedbySelf _asbp_base_collectable))
    (:CastFailed
      _))
  (return (Variables|/Script/Engine.SoundBase|GetDuration _sound)))