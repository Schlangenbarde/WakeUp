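; Base collection actor that tracks a set of collectables in a level and keeps their collected state across saves.
; On BeginPlay it loads this level's entry from the save slot, destroys already collected items and binds to each collectable's collected event.
; Each pickup records its index in the shrinking array, removes it and updates an existing save, keyed by level name.
; An empty array fires OnAllCollected, including after a short startup delay.
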(event Custom|CustomEvent
  (params (From :type BP%20Base%20Collectable%20Object%20Reference))
  (bind _collecables (Variables|Default|GetCollecables))
  (Utilities|Array|Add (Variables|Default|GetCollection%20Of%20Collectables) (Utilities|Struct|MakeSTRUCT_Collectable (Utilities|Array|FindItem _collecables From) true))
  (Utilities|Array|RemoveItem _collecables From)
  (CallFunction|SaveData)
  (bind _result (CallFunction|IsLessThan0 (Variables|Default|GetCollecables)))
  (if _result
    (Default|CallOnAllCollected)))

(event EventBeginPlay
  (CallFunction|LoadData)
  (for _array_element (Variables|Default|GetCollecables)
    (EventDispatchers|BindEventtoOnCollectedbySelf _array_element (EventDispatchers|CreateEvent :!event Custom|CustomEvent)))
  (Utilities|FlowControl|Delay 0.5)
  (bind _result (CallFunction|IsLessThan0 (Variables|Default|GetCollecables)))
  (if _result
    (Default|CallOnAllCollected)))

(fn ConstructionScript)

(fn IsLessThan0
  (params (TargetArray :type Array%20of%20BP%20Base%20Collectable%20Object%20References))
  (return (<= (Utilities|Array|Length TargetArray) 0)))

(fn LoadData
  (bind _collecables (Variables|Default|GetCollecables))
  (bind _returnvalue (SaveGame|DoesSaveGameExist "MyCoolSlot"))
  (if _returnvalue
    (bind _returnvalue_2 (SaveGame|LoadGamefromSlot "MyCoolSlot"))
    (bind _asbp_save_game_save_slot_one (Utilities|Casting|CastToBP_SaveGame_SaveSlotOne _returnvalue_2))
    (bind _returnvalue_3 (Game|GetCurrentLevelName true))
    (for _array_element (Variables|/Game/Data/SaveClasses/BP_SaveGame_SaveSlotOne.BP_SaveGame_SaveSlotOne_C|GetCollectionOfCollectables _asbp_save_game_save_slot_one)
      (if (== (Utilities|String|StringToName _returnvalue_3) (Utilities|String|StringToName (.levelname _array_element)))
        (for _array_element_2 (.structcollectable _array_element)
          (if (.gotcollectet _array_element_2)
            (Actor|DestroyActor (Utilities|Array|Get(acopy) _collecables (.index _array_element_2)))
            (Utilities|Array|RemoveItem _collecables (Utilities|Array|Get(acopy) _collecables (.index _array_element_2)))))
        (Variables|Default|SetCollection%20Of%20Collectables (.structcollectable _array_element))
        (return)))))

(fn SaveData
  (bind _collection_of_collectables (Variables|Default|GetCollection%20Of%20Collectables))
  (bind _returnvalue (SaveGame|DoesSaveGameExist "MyCoolSlot"))
  (if _returnvalue
    (bind _returnvalue_2 (SaveGame|LoadGamefromSlot "MyCoolSlot"))
    (bind _asbp_save_game_save_slot_one (Utilities|Casting|CastToBP_SaveGame_SaveSlotOne _returnvalue_2))
    (bind _returnvalue_3 (Game|GetCurrentLevelName true))
    (for (_array_element _array_index) (Variables|/Game/Data/SaveClasses/BP_SaveGame_SaveSlotOne.BP_SaveGame_SaveSlotOne_C|GetCollectionOfCollectables _asbp_save_game_save_slot_one)
      (if (== (Utilities|String|StringToName (.levelname _array_element)) (Utilities|String|StringToName _returnvalue_3))
        (Utilities|Array|SetArrayElem (Variables|/Game/Data/SaveClasses/BP_SaveGame_SaveSlotOne.BP_SaveGame_SaveSlotOne_C|GetCollectionOfCollectables _asbp_save_game_save_slot_one) _array_index (Utilities|Struct|MakeSTRUCT_CollectionOfCollectables (.levelname _array_element) _collection_of_collectables))
        (SaveGame|SaveGametoSlot _returnvalue_2 "MyCoolSlot")
        (return)))
    (Utilities|Array|Add (Variables|/Game/Data/SaveClasses/BP_SaveGame_SaveSlotOne.BP_SaveGame_SaveSlotOne_C|GetCollectionOfCollectables _asbp_save_game_save_slot_one) (Utilities|Struct|MakeSTRUCT_CollectionOfCollectables _returnvalue_3 _collection_of_collectables))
    (SaveGame|SaveGametoSlot _returnvalue_2 "MyCoolSlot")))